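; BP_Phonebox is an interactable phone box that rings and opens a phone conversation through DialoguePhone.
; The ringing event starts Wwise audio when DialoguePhone reports ready, and Tick drives the TelephoneFade RTPC from player distance while it plays.
; Interact stops the ring, plays a pickup sound and sets a Wwise state, with a separate one for the final call.
; ConversationClosed notifies the stored instigator.
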(event `self.Interact`
  (params (Instigator :type "Actor Object Reference"))
  (set `self.InteractactableInstigator` Instigator)
  (`/Game/Blueprints/AC_dialogue_base.OpenConversation` (`self.Dialogue_Phone`))
  (`self.StopPhoneAudio`)
  (`AkGameplayStatics.PostEvent` "/Game/WwiseAudio/Events/Default_Work_Unit/PhonePickup.PhonePickup")
  (if (`/Game/Blueprints/Dialogue_Phone.IsLastPhoneCall` (`self.Dialogue_Phone`))
    (`AkGameplayStatics.SetState` "/Game/WwiseAudio/States/MUSIC/Game_state/Game_state-Phone_final.Game_state-Phone_final")
    (else
      (`AkGameplayStatics.SetState` "/Game/WwiseAudio/States/MUSIC/Game_state/Game_state-Phone.Game_state-Phone"))))

(event `ringing`
  (bind _readytophone (`/Game/Blueprints/AC_dialogue_base.GetIsReadyToPhoneBool` (`self.Dialogue_Phone`)))
  (if _readytophone
    (`self.StartPhoneAudio`)))

(event `self.ReceiveTick`
  (params (DeltaSeconds :type "Float (single-precision)"))
  (if (`self.isPlaying`)
    (bind _r (`self.InverseLerp` 1000.0 100.0 (`self.GetDistanceTo` (`GameplayStatics.GetPlayerPawn` 0))))
    (`AkGameplayStatics.SetRTPCValue` "/Game/WwiseAudio/Game_Parameters/Default_Work_Unit/TelephoneFade.TelephoneFade" _r)))

(event `self.ConversationClosed`
  (message `/Game/Blueprints/BPI_Interactable.ConversationClosed` (`self.InteractactableInstigator`)))

(fn `InverseLerp`
  (params (A :type "Float (double-precision)") (B :type "Float (double-precision)") (V :type "Float (double-precision)"))
  (returns (R :type "Float (double-precision)"))
  (return (`KismetMathLibrary.FClamp` (/ (- V A) (- B A)))))

(fn `StartPhoneAudio`
  (set `self.isPlaying` true)
  (`AkGameplayStatics.PostEvent` "/Game/WwiseAudio/TelephoneBox/TelephoneStart.TelephoneStart"))

(fn `StopPhoneAudio`
  (`AkGameplayStatics.PostEvent` "/Game/WwiseAudio/Events/Default_Work_Unit/TelephoneStop.TelephoneStop")
  (set `self.isPlaying` false))

(fn `UserConstructionScript`)