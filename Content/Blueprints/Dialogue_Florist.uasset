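; Dialogue Blueprint for the Florist NPC, an elderly shopkeeper who cautiously voices discontent with the State through branching player choices.
; It extends the parent Dialogue function, gating on phone readiness, level progress and tree index, with nested AddDialogue nodes whose branches reconverge on shared lines.
; Early exits save a tree index, while the full confession fires a Lightbulb Wwise event, advances level progress and rings BP_Phonebox for the player to report in.
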(fn `Dialogue`
  (`parent.Dialogue`)
  (bind _readytophone (`self.GetIsReadyToPhoneBool`))
  (if _readytophone
    (bind _state (`self.AddDialogue` "You" "I should report in at the phone." (`|MakeArray` "[Close]" :!type "Text")))
    (switch `/Game/Blueprints/Enum_DialogueState` _state
      (:`NewEnumerator0`
        (`self.ClearDialogueProgress`)
        (`self.CloseConversation`)))
    (else
      (bind _this_index (`self.GetLevelProgressIndex`))
      (switch `int` _this_index
        (:`0`
          (switch `int` (`self.DialogueTreeIndex`)
            (:`0`
              (bind _state_2 (`self.AddDialogue` "Florist" "Oh... Pleasantries, young man." (`|MakeArray` "Hello" "Pleasantries" :!type "Text")))
              (switch `/Game/Blueprints/Enum_DialogueState` _state_2
                (:`NewEnumerator0`
                  (bind (_state_3 _optionindex) (`self.AddDialogue` "Florist" "Blessed morning we're having." (`|MakeArray` "How are you today?" "Busy day?" :!type "Text")))
                  (switch `/Game/Blueprints/Enum_DialogueState` _state_3
                    (:`NewEnumerator0`
                      (switch `int` _optionindex
                        (:`0`
                          (bind _state_4 (`self.AddDialogue` "Florist" "Goodness, there's a rare question." (`|MakeArray` "[Next]" :!type "Text")))
                          (switch `/Game/Blueprints/Enum_DialogueState` _state_4
                            (:`NewEnumerator0`
                              (bind (_state_5 _optionindex_2) (`self.AddDialogue` "Florist" "I’m fine… The same as every other day, I suppose." (`|MakeArray` "You're a florist?" "Nice shop you have here" :!type "Text")))
                              (switch `/Game/Blueprints/Enum_DialogueState` _state_5
                                (:`NewEnumerator0`
                                  (switch `int` _optionindex_2
                                    (:`0`
                                      (bind _state_6 (`self.AddDialogue` "Florist" "Since my retirement, yes." (`|MakeArray` "[Next]" :!type "Text")))
                                      (switch `/Game/Blueprints/Enum_DialogueState` _state_6
                                        (:`NewEnumerator0`
                                          (bind _state_7 (`self.AddDialogue` "Florist" "My mother...she was the real florist." (`|MakeArray` "[Next]" :!type "Text")))
                                          (switch `/Game/Blueprints/Enum_DialogueState` _state_7
                                            (:`NewEnumerator0`
                                              (bind _state_8 (`self.AddDialogue` "Florist" "I still remember her little shop... " (`|MakeArray` "[Next]" :!type "Text")))
                                              (switch `/Game/Blueprints/Enum_DialogueState` _state_8
                                                (:`NewEnumerator0`
                                                  (bind (_state_9 _optionindex_3) (`self.AddDialogue` "Florist" "I used to read in the back as a girl." (`|MakeArray` "You 'retired' into more work?" "Is it like you imagined as a kid?" :!type "Text")))
                                                  (switch `/Game/Blueprints/Enum_DialogueState` _state_9
                                                    (:`NewEnumerator0`
                                                      (switch `int` _optionindex_3
                                                        (:`0`
                                                          (bind _state_10 (`self.AddDialogue` "Florist" "As we all do... but I count myself lucky." (`|MakeArray` "[Next]" :!type "Text")))
                                                          (switch `/Game/Blueprints/Enum_DialogueState` _state_10
                                                            (:`NewEnumerator0`
                                                              (bind (_state_11 _optionindex_4) (`self.AddDialogue` "Florist" "My knees couldn’t handle much else." (`|MakeArray` "And the unlucky ones?" "Well the flowers you have are uhh..." :!type "Text")))
                                                              (switch `/Game/Blueprints/Enum_DialogueState` _state_11
                                                                (:`NewEnumerator0`
                                                                  (switch `int` _optionindex_4
                                                                    (:`0`
                                                                      (bind _state_12 (`self.AddDialogue` "Florist" "They were... re-assigned." (`|MakeArray` "[Next]" :!type "Text")))
                                                                      (switch `/Game/Blueprints/Enum_DialogueState` _state_12
                                                                        (:`NewEnumerator0`
                                                                          (bind _state_13 (`self.AddDialogue` "Florist" "You know I really should be going now, Sir." (`|MakeArray` "[Next]" :!type "Text")))
                                                                          (switch `/Game/Blueprints/Enum_DialogueState` _state_13
                                                                            (:`NewEnumerator0`
                                                                              (bind _state_14 (`self.AddDialogue` "Florist" "You have a nice-" (`|MakeArray` "[Next]" :!type "Text")))
                                                                              (switch `/Game/Blueprints/Enum_DialogueState` _state_14
                                                                                (:`NewEnumerator0`
                                                                                  (bind _state_15 (`self.AddDialogue` "Florist" "A pleasant day." (`|MakeArray` "[Next]" :!type "Text")))
                                                                                  (switch `/Game/Blueprints/Enum_DialogueState` _state_15
                                                                                    (:`NewEnumerator0`
                                                                                      (`self.SetDialogueTreeIndex` 1)
                                                                                      (`self.ClearDialogueProgress`)
                                                                                      (`self.CloseConversation`))))))))))
                                                                    (:`1`
                                                                      (bind _state_16 (`self.AddDialogue` "Florist" "Mm, the State approved palette." (`|MakeArray` "[Next]" :!type "Text") :!label _label))
                                                                      (switch `/Game/Blueprints/Enum_DialogueState` _state_16
                                                                        (:`NewEnumerator0`
                                                                          (bind (_state_17 _optionindex_5) (`self.AddDialogue` "Florist" "‘Harmony through uniformity’. That’s the slogan, isn’t it? " (`|MakeArray` "You must miss all the diversity" "How long has it been like this?" :!type "Text")))
                                                                          (switch `/Game/Blueprints/Enum_DialogueState` _state_17
                                                                            (:`NewEnumerator0`
                                                                              (switch `int` _optionindex_5
                                                                                (:`0`
                                                                                  (bind _state_18 (`self.AddDialogue` "Florist" "..." (`|MakeArray` "[Next]" :!type "Text") :!label _label_2))
                                                                                  (switch `/Game/Blueprints/Enum_DialogueState` _state_18
                                                                                    (:`NewEnumerator0`
                                                                                      (bind _state_19 (`self.AddDialogue` "Florist" "Yes, I do. Though most never noticed... " (`|MakeArray` "[Next]" :!type "Text")))
                                                                                      (switch `/Game/Blueprints/Enum_DialogueState` _state_19
                                                                                        (:`NewEnumerator0`
                                                                                          _)))))
                                                                                (:`1`
                                                                                  (bind _state_20 (`self.AddDialogue` "Florist" "...Long enough that people stopped asking for non-State colours." (`|MakeArray` "[Next]" :!type "Text") :!label _label_3))
                                                                                  (switch `/Game/Blueprints/Enum_DialogueState` _state_20
                                                                                    (:`NewEnumerator0`
                                                                                      _))))
                                                                              (bind _state_21 (`self.AddDialogue` "Florist" "It’s as if the world faded one colour at a time, and no one said a word." (`|MakeArray` "I'm sorry..." "But you haven't forgotten" "How disturbing" :!type "Text")))
                                                                              (switch `/Game/Blueprints/Enum_DialogueState` _state_21
                                                                                (:`NewEnumerator0`
                                                                                  (bind (_state_22 _optionindex_6) (`self.AddDialogue` "Florist" "Gracious, don’t listen to me. I’m just a bitter old woman." (`|MakeArray` "No, please continue" "I'd like to hear the rest" "Yes we should stop" :!type "Text")))
                                                                                  (switch `/Game/Blueprints/Enum_DialogueState` _state_22
                                                                                    (:`NewEnumerator0`
                                                                                      (switch `int` _optionindex_6
                                                                                        (:`0`
                                                                                          (bind _state_23 (`self.AddDialogue` "Florist" "You know… in all those years working the fields" (`|MakeArray` "[Next]" :!type "Text") :!label _label_4))
                                                                                          (switch `/Game/Blueprints/Enum_DialogueState` _state_23
                                                                                            (:`NewEnumerator0`
                                                                                              (bind _state_24 (`self.AddDialogue` "Florist" "I used to imagine what it would feel like to spend my day bringing colour back into people’s lives. " (`|MakeArray` "[Next]" :!type "Text")))
                                                                                              (switch `/Game/Blueprints/Enum_DialogueState` _state_24
                                                                                                (:`NewEnumerator0`
                                                                                                  (bind _state_25 (`self.AddDialogue` "Florist" "Just a little vase on the mantle... the passing scent of a rose..." (`|MakeArray` "[Next]" :!type "Text")))
                                                                                                  (switch `/Game/Blueprints/Enum_DialogueState` _state_25
                                                                                                    (:`NewEnumerator0`
                                                                                                      (bind _state_26 (`self.AddDialogue` "Florist" "It may seem a silly thought, but these things matter." (`|MakeArray` "[Next]" :!type "Text")))
                                                                                                      (switch `/Game/Blueprints/Enum_DialogueState` _state_26
                                                                                                        (:`NewEnumerator0`
                                                                                                          (bind _state_27 (`self.AddDialogue` "Florist" "They bring joy. Simple pleasures. But the State..." (`|MakeArray` "Sees no value in it?" "Wouldn't allow you?" :!type "Text")))
                                                                                                          (switch `/Game/Blueprints/Enum_DialogueState` _state_27
                                                                                                            (:`NewEnumerator0`
                                                                                                              (bind _state_28 (`self.AddDialogue` "Florist" "Forgive me...I really ought to stop." (`|MakeArray` "[Next]" :!type "Text")))
                                                                                                              (switch `/Game/Blueprints/Enum_DialogueState` _state_28
                                                                                                                (:`NewEnumerator0`
                                                                                                                  (bind _state_29 (`self.AddDialogue` "Florist" "I’m sure you’ve noticed the statue over the way." (`|MakeArray` "[Next]" :!type "Text")))
                                                                                                                  (switch `/Game/Blueprints/Enum_DialogueState` _state_29
                                                                                                                    (:`NewEnumerator0`
                                                                                                                      (bind _state_30 (`self.AddDialogue` "Florist" "The Architect, himself, our 'Saviour'... always watching." (`|MakeArray` "[Next]" :!type "Text")))
                                                                                                                      (switch `/Game/Blueprints/Enum_DialogueState` _state_30
                                                                                                                        (:`NewEnumerator0`
                                                                                                                          (bind _state_31 (`self.AddDialogue` "Florist" "Ready to turn us all into Heretics... I'm nearly ninety years old, and even now I'm still a threat. What a sad sad man." (`|MakeArray` "[Next]" :!type "Text")))
                                                                                                                          (switch `/Game/Blueprints/Enum_DialogueState` _state_31
                                                                                                                            (:`NewEnumerator0`
                                                                                                                              (`AkGameplayStatics.PostEvent` "/Game/WwiseAudio/Events/MUSIC/Lightbulb.Lightbulb")
                                                                                                                              (bind (_state_32 _optionindex_7) (`self.AddDialogue` "Florist" "All of this...stays between us I hope?" (`|MakeArray` "Of course" "Umm..." :!type "Text")))
                                                                                                                              (switch `/Game/Blueprints/Enum_DialogueState` _state_32
                                                                                                                                (:`NewEnumerator0`
                                                                                                                                  (switch `int` _optionindex_7
                                                                                                                                    (:`0`
                                                                                                                                      (bind _state_33 (`self.AddDialogue` "Florist" "Wonderful. Trust is hard to come by these days..." (`|MakeArray` "[Next]" :!type "Text")))
                                                                                                                                      (switch `/Game/Blueprints/Enum_DialogueState` _state_33
                                                                                                                                        (:`NewEnumerator0`
                                                                                                                                          (bind _state_34 (`self.AddDialogue` "Florist" "Please- you’ll have to excuse me... Pleasant day, Sir." (`|MakeArray` "[Close]" :!type "Text")))
                                                                                                                                          (switch `/Game/Blueprints/Enum_DialogueState` _state_34
                                                                                                                                            (:`NewEnumerator0`
                                                                                                                                              (`self.SetLevelProgressIndex` 1)
                                                                                                                                              (`self.SetIsReadyToPhoneBool` true)
                                                                                                                                              (`self.ClearDialogueProgress`)
                                                                                                                                              (`self.CloseConversation`)
                                                                                                                                              (bind _returnvalue (`GameplayStatics.GetActorOfClass` "/Game/Models/BP_Phonebox.BP_Phonebox_C"))
                                                                                                                                              (`/Game/Models/BP_Phonebox.ringing` _returnvalue))))))
                                                                                                                                    (:`1`
                                                                                                                                      (bind _state_35 (`self.AddDialogue` "Florist" "..." (`|MakeArray` "[Next]" :!type "Text")))
                                                                                                                                      (switch `/Game/Blueprints/Enum_DialogueState` _state_35
                                                                                                                                        (:`NewEnumerator0`
                                                                                                                                          (bind _state_36 (`self.AddDialogue` "Florist" "Oh dear what have I done..." (`|MakeArray` "[Next]" :!type "Text")))
                                                                                                                                          (switch `/Game/Blueprints/Enum_DialogueState` _state_36
                                                                                                                                            (:`NewEnumerator0`
                                                                                                                                              (bind _state_37 (`self.AddDialogue` "Florist" "Please- excuse me... Goodbye." (`|MakeArray` "[Close]" :!type "Text")))
                                                                                                                                              (switch `/Game/Blueprints/Enum_DialogueState` _state_37
                                                                                                                                                (:`NewEnumerator0`
                                                                                                                                                  (`self.SetLevelProgressIndex` 1)
                                                                                                                                                  (`self.SetIsReadyToPhoneBool` true)
                                                                                                                                                  (`self.ClearDialogueProgress`)
                                                                                                                                                  (`self.CloseConversation`)
                                                                                                                                                  (bind _returnvalue_2 (`GameplayStatics.GetActorOfClass` "/Game/Models/BP_Phonebox.BP_Phonebox_C"))
                                                                                                                                                  (`/Game/Models/BP_Phonebox.ringing` _returnvalue_2))))))))))))))))))))))))))))))
                                                                                        (:`1`
                                                                                          (goto _label_4))
                                                                                        (:`2`
                                                                                          (bind _state_38 (`self.AddDialogue` "Florist" "Y-yes of course." (`|MakeArray` "[Next]" :!type "Text")))
                                                                                          (switch `/Game/Blueprints/Enum_DialogueState` _state_38
                                                                                            (:`NewEnumerator0`
                                                                                              (bind _state_39 (`self.AddDialogue` "Florist" "You know I really should be going now, Sir." (`|MakeArray` "[Next]" :!type "Text")))
                                                                                              (switch `/Game/Blueprints/Enum_DialogueState` _state_39
                                                                                                (:`NewEnumerator0`
                                                                                                  (bind _state_40 (`self.AddDialogue` "Florist" "You have a nice-" (`|MakeArray` "[Next]" :!type "Text")))
                                                                                                  (switch `/Game/Blueprints/Enum_DialogueState` _state_40
                                                                                                    (:`NewEnumerator0`
                                                                                                      (bind _state_41 (`self.AddDialogue` "Florist" "A pleasant day." (`|MakeArray` "[Next]" :!type "Text")))
                                                                                                      (switch `/Game/Blueprints/Enum_DialogueState` _state_41
                                                                                                        (:`NewEnumerator0`
                                                                                                          (`self.SetDialogueTreeIndex` 2)
                                                                                                          (`self.ClearDialogueProgress`)
                                                                                                          (`self.CloseConversation`))))))))))))))))))))))))))
                                                        (:`1`
                                                          (bind (_state_42 _optionindex_8) (`self.AddDialogue` "Florist" "Admittedly, times were different back then. Mum sold more... variety. " (`|MakeArray` "You must miss all the diversity" "How long has it been like this?" :!type "Text")))
                                                          (switch `/Game/Blueprints/Enum_DialogueState` _state_42
                                                            (:`NewEnumerator0`
                                                              (switch `int` _optionindex_8
                                                                (:`0`
                                                                  (goto _label_2))
                                                                (:`1`
                                                                  (goto _label_3))))))))))))))))
                                    (:`1`
                                      (bind _state_43 (`self.AddDialogue` "Florist" "Why, thank you. We do what we can." (`|MakeArray` "[Next]" :!type "Text")))
                                      (switch `/Game/Blueprints/Enum_DialogueState` _state_43
                                        (:`NewEnumerator0`
                                          (bind _state_44 (`self.AddDialogue` "Florist" "The State likes things… neat. As I'm sure you know." (`|MakeArray` "Well the flowers you have are uhh..." "You only sell grey and white?" :!type "Text")))
                                          (switch `/Game/Blueprints/Enum_DialogueState` _state_44
                                            (:`NewEnumerator0`
                                              (goto _label))))))))))))
                        (:`1`
                          (bind (_state_45 _optionindex_9) (`self.AddDialogue` "Florist" "Rather quiet actually. Not much on offer, I’m afraid." (`|MakeArray` "Why's that?" "I noticed you only sell grey and white flowers" :!type "Text")))
                          (switch `/Game/Blueprints/Enum_DialogueState` _state_45
                            (:`NewEnumerator0`
                              (switch `int` _optionindex_9
                                (:`0`
                                  (bind (_state_46 _optionindex_10) (`self.AddDialogue` "Florist" "Supply shortage I’m told... You know what they say." (`|MakeArray` "Has it been a problem for a while?" "No fault of your own" :!type "Text")))
                                  (switch `/Game/Blueprints/Enum_DialogueState` _state_46
                                    (:`NewEnumerator0`
                                      (switch `int` _optionindex_10
                                        (:`0`
                                          (bind (_state_47 _optionindex_11) (`self.AddDialogue` "Florist" "Grey... White... The only flowers I’m receive these days... The State’s colours." (`|MakeArray` "You must miss all the diversity." "How long has it been like this?" :!type "Text") :!label _label_5))
                                          (switch `/Game/Blueprints/Enum_DialogueState` _state_47
                                            (:`NewEnumerator0`
                                              (switch `int` _optionindex_11
                                                (:`0`
                                                  (goto _label_2))
                                                (:`1`
                                                  (goto _label_3))))))
                                        (:`1`
                                          (bind (_state_48 _optionindex_12) (`self.AddDialogue` "Florist" "Well fault is a funny little thing, isn’t it… Doesn’t spare you from the consequences." (`|MakeArray` "Consequences?" "Sounds like the State's been letting you down" :!type "Text")))
                                          (switch `/Game/Blueprints/Enum_DialogueState` _state_48
                                            (:`NewEnumerator0`
                                              (switch `int` _optionindex_12
                                                (:`0`
                                                  (goto _label_5))
                                                (:`1`
                                                  (bind _state_49 (`self.AddDialogue` "Florist" "..." (`|MakeArray` "[Next]" :!type "Text")))
                                                  (switch `/Game/Blueprints/Enum_DialogueState` _state_49
                                                    (:`NewEnumerator0`
                                                      (bind _state_50 (`self.AddDialogue` "Florist" "No- no, of course not" (`|MakeArray` "[Next]" :!type "Text")))
                                                      (switch `/Game/Blueprints/Enum_DialogueState` _state_50
                                                        (:`NewEnumerator0`
                                                          (bind _state_51 (`self.AddDialogue` "Florist" "No- no, of course not" (`|MakeArray` "[Next]" :!type "Text")))
                                                          (switch `/Game/Blueprints/Enum_DialogueState` _state_51
                                                            (:`NewEnumerator0`
                                                              (`self.SetDialogueTreeIndex` 1)
                                                              (`self.ClearDialogueProgress`)
                                                              (`self.CloseConversation`))))))))))))))))
                                (:`1`
                                  (goto _label))))))))))))
            (:`1`
              (bind (_state_52 _optionindex_13) (`self.AddDialogue` "Florist" "Hello dear, was there something else you needed?" (`|MakeArray` "Nothing, nevermind" "Do you have anything other than grey and white flowers?" :!type "Text")))
              (switch `/Game/Blueprints/Enum_DialogueState` _state_52
                (:`NewEnumerator0`
                  (switch `int` _optionindex_13
                    (:`0`
                      (`self.ClearDialogueProgress`)
                      (`self.CloseConversation`))
                    (:`1`
                      (goto _label))))))
            (:`2`
              (bind (_state_53 _optionindex_14) (`self.AddDialogue` "Florist" "...Yes, dear?" (`|MakeArray` "Nothing, nevermind" "I'm sorry, tell me more " :!type "Text")))
              (switch `/Game/Blueprints/Enum_DialogueState` _state_53
                (:`NewEnumerator0`
                  (switch `int` _optionindex_14
                    (:`0`
                      (`self.ClearDialogueProgress`)
                      (`self.CloseConversation`))
                    (:`1`
                      (bind _state_54 (`self.AddDialogue` "Florist" "Are you sure you wish to know?" (`|MakeArray` "Yes, I'm sure" "I would like nothing more " :!type "Text")))
                      (switch `/Game/Blueprints/Enum_DialogueState` _state_54
                        (:`NewEnumerator0`
                          (bind _state_55 (`self.AddDialogue` "Florist" "Well aright then." (`|MakeArray` "[Next]" :!type "Text")))
                          (switch `/Game/Blueprints/Enum_DialogueState` _state_55
                            (:`NewEnumerator0`
                              (goto _label_4))))))))))))
        (:`1`
          (switch `int` (`self.DialogueTreeIndex`) :!label _label_6
            (:`0`
              (bind _state_56 (`self.AddDialogue` "Florist" "Pleasantries young man. Blessed day!" (`|MakeArray` "Are you alright?" "Did anyone... speak to you?" :!type "Text") :!label _label_7))
              (switch `/Game/Blueprints/Enum_DialogueState` _state_56
                (:`NewEnumerator0`
                  (bind _state_57 (`self.AddDialogue` "Florist" "We’ve got a gorgeous selection of flowers today, just gorgeous!  Grey, white- here, come, have a look!" (`|MakeArray` "Don’t you remember me?" "You seem, different?" :!type "Text")))
                  (switch `/Game/Blueprints/Enum_DialogueState` _state_57
                    (:`NewEnumerator0`
                      (bind _state_58 (`self.AddDialogue` "Florist" "The State really does have an eye for colour! What can I prepare for you? Don’t be shy." (`|MakeArray` "What's happened to you..." "Did I do this?" :!type "Text")))
                      (switch `/Game/Blueprints/Enum_DialogueState` _state_58
                        (:`NewEnumerator0`
                          (bind _state_59 (`self.AddDialogue` "Florist" "We also sell a variety of vase and pot options-" (`|MakeArray` "...I should get going" "..." :!type "Text")))
                          (switch `/Game/Blueprints/Enum_DialogueState` _state_59
                            (:`NewEnumerator0`
                              (`self.SetDialogueTreeIndex` 2)
                              (`self.ClearDialogueProgress`)
                              (`self.CloseConversation`))))))))))
            (:`1`
              (goto _label_7))
            (:`2`
              (bind (_state_60 _optionindex_15) (`self.AddDialogue` "Florist" "Pleasantries young man. Blessed day!" (`|MakeArray` "..." "[Close]" :!type "Text")))
              (switch `/Game/Blueprints/Enum_DialogueState` _state_60
                (:`NewEnumerator0`
                  (switch `int` _optionindex_15
                    (:`0`
                      (bind (_state_61 _optionindex_16) (`self.AddDialogue` "Florist" "We’ve got a gorgeous selection of flowers today, just gorgeous!  Grey, white- here, come, have a look!" (`|MakeArray` "I'm sorry..." "[Close]" :!type "Text")))
                      (switch `/Game/Blueprints/Enum_DialogueState` _state_61
                        (:`NewEnumerator0`
                          (switch `int` _optionindex_16
                            (:`0`
                              (bind _state_62 (`self.AddDialogue` "Florist" "The State really does have an eye for colour! What can I prepare for you? Don’t be shy." (`|MakeArray` "[Close]" :!type "Text")))
                              (switch `/Game/Blueprints/Enum_DialogueState` _state_62
                                (:`NewEnumerator0`
                                  (`self.ClearDialogueProgress`)
                                  (`self.CloseConversation`))))
                            (:`1`
                              (`self.ClearDialogueProgress`)
                              (`self.CloseConversation`))))))
                    (:`1`
                      (`self.ClearDialogueProgress`)
                      (`self.CloseConversation`))))))))
        (:`2`
          (goto _label_6))))))