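; Dialogue script for the Heretic NPC, a speaker who replies only in ellipses and emoticons.
; It overrides the parent Dialogue function, chaining AddDialogue nodes whose option choices branch the conversation.
; A ready-to-phone check preempts the talk; otherwise level progress and a saved DialogueTreeIndex pick the tree.
; Levels 0 and 1 share a tree, while level 2 renames the speaker in quotes and records a kind or cruel ending.
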(fn `Dialogue`
  (`parent.Dialogue`)
  (bind _readytophone (`self.GetIsReadyToPhoneBool`))
  (if _readytophone
    (bind _state (`self.AddDialogue` "You" "I should report in at the phone." (`|MakeArray` "[Close]" :!type "Text")))
    (switch `/Game/Blueprints/Enum_DialogueState` _state
      (:`NewEnumerator0`
        (`self.ClearDialogueProgress`)
        (`self.CloseConversation`)))
    (else
      (bind _this_index (`self.GetLevelProgressIndex`))
      (switch `int` _this_index
        (:`0`
          (switch `int` (`self.DialogueTreeIndex`) :!label _label
            (:`0`
              (bind (_state_2 _optionindex) (`self.AddDialogue` "A Heretic" "..." (`|MakeArray` "Pleasantries" "..." :!type "Text")))
              (switch `/Game/Blueprints/Enum_DialogueState` _state_2
                (:`NewEnumerator0`
                  (switch `int` _optionindex
                    (:`0`
                      (bind _state_3 (`self.AddDialogue` "A Heretic" "....." (`|MakeArray` "Umm.." "Are you ok?" :!type "Text")))
                      (switch `/Game/Blueprints/Enum_DialogueState` _state_3
                        (:`NewEnumerator0`
                          (bind _state_4 (`self.AddDialogue` "A Heretic" "............" (`|MakeArray` (select `int` (`KismetMathLibrary.RandomIntegerInRange` 0 1) :`0` "Ok..." :`1` "Alright then.." :!type "Text"))))
                          (switch `/Game/Blueprints/Enum_DialogueState` _state_4
                            (:`NewEnumerator0`
                              (`self.SetDialogueTreeIndex` 1)
                              (`self.ClearDialogueProgress`)
                              (`self.CloseConversation`))))))
                    (:`1`
                      (bind _state_5 (`self.AddDialogue` "A Heretic" "....." (`|MakeArray` "........" "..............." :!type "Text")))
                      (switch `/Game/Blueprints/Enum_DialogueState` _state_5
                        (:`NewEnumerator0`
                          (bind (_state_6 _optionindex_2) (`self.AddDialogue` "A Heretic" "............." (`|MakeArray` "(I'm sorry)" "......................" :!type "Text")))
                          (switch `/Game/Blueprints/Enum_DialogueState` _state_6
                            (:`NewEnumerator0`
                              (switch `int` _optionindex_2
                                (:`0`
                                  (bind _state_7 (`self.AddDialogue` "A Heretic" "....... :')" (`|MakeArray` "Close" :!type "Text")))
                                  (switch `/Game/Blueprints/Enum_DialogueState` _state_7
                                    (:`NewEnumerator0`
                                      (`self.SetDialogueTreeIndex` 1)
                                      (`self.ClearDialogueProgress`)
                                      (`self.CloseConversation`))))
                                (:`1`
                                  (bind _state_8 (`self.AddDialogue` "A Heretic" "......." (`|MakeArray` "Close" :!type "Text")))
                                  (switch `/Game/Blueprints/Enum_DialogueState` _state_8
                                    (:`NewEnumerator0`
                                      (`self.ClearDialogueProgress`)
                                      (`self.CloseConversation`))))))))))))))
            (:`1`
              (bind (_state_9 _optionindex_3) (`self.AddDialogue` "A Heretic" "..." (`|MakeArray` "Hello again" "..." :!type "Text")))
              (switch `/Game/Blueprints/Enum_DialogueState` _state_9
                (:`NewEnumerator0`
                  (switch `int` _optionindex_3
                    (:`0`
                      (bind _state_10 (`self.AddDialogue` "A Heretic" "...." (`|MakeArray` "How long have they made you stand here..." "You must be hungry" :!type "Text")))
                      (switch `/Game/Blueprints/Enum_DialogueState` _state_10
                        (:`NewEnumerator0`
                          _)))
                    (:`1`
                      (bind _state_11 (`self.AddDialogue` "A Heretic" "...." (`|MakeArray` "Your mouth must hurt" "..." :!type "Text")))
                      (switch `/Game/Blueprints/Enum_DialogueState` _state_11
                        (:`NewEnumerator0`
                          _))))
                  (bind (_state_12 _optionindex_4) (`self.AddDialogue` "A Heretic" "......." (`|MakeArray` "I don't think I can help you though" "Maybe I'll look into getting you something..." :!type "Text")))
                  (switch `/Game/Blueprints/Enum_DialogueState` _state_12
                    (:`NewEnumerator0`
                      (switch `int` _optionindex_4
                        (:`0`
                          (bind _state_13 (`self.AddDialogue` "A Heretic" "......... :(" (`|MakeArray` "[Close]" :!type "Text")))
                          (switch `/Game/Blueprints/Enum_DialogueState` _state_13
                            (:`NewEnumerator0`
                              (`self.SetDialogueTreeIndex` 2)
                              (`self.ClearDialogueProgress`)
                              (`self.CloseConversation`))))
                        (:`1`
                          (bind _state_14 (`self.AddDialogue` "A Heretic" ".......... :)" (`|MakeArray` "[Close]" :!type "Text")))
                          (switch `/Game/Blueprints/Enum_DialogueState` _state_14
                            (:`NewEnumerator0`
                              (`self.SetDialogueTreeIndex` 2)
                              (`self.ClearDialogueProgress`)
                              (`self.CloseConversation`))))))))))
            (:`2`
              (bind _state_15 (`self.AddDialogue` "A Heretic" "..." (`|MakeArray` "I'll come back tomorrow, promise" "..." :!type "Text")))
              (switch `/Game/Blueprints/Enum_DialogueState` _state_15
                (:`NewEnumerator0`
                  (bind _state_16 (`self.AddDialogue` "A Heretic" ".... :')" (`|MakeArray` "[Close]" :!type "Text")))
                  (switch `/Game/Blueprints/Enum_DialogueState` _state_16
                    (:`NewEnumerator0`
                      (`self.ClearDialogueProgress`)
                      (`self.CloseConversation`))))))))
        (:`1`
          (goto _label))
        (:`2`
          (switch `int` (`self.DialogueTreeIndex`)
            (:`0`
              (bind _state_17 (`self.AddDialogue` "A \"Heretic\"" "....." (`|MakeArray` "........" "Sorry I didn't bring you anything" :!type "Text") :!label _label_2))
              (switch `/Game/Blueprints/Enum_DialogueState` _state_17
                (:`NewEnumerator0`
                  (bind (_state_18 _optionindex_5) (`self.AddDialogue` "A \"Heretic\"" "............." (`|MakeArray` "I'll stop this from ever happening again" "You got what was coming" :!type "Text")))
                  (switch `/Game/Blueprints/Enum_DialogueState` _state_18
                    (:`NewEnumerator0`
                      (switch `int` _optionindex_5
                        (:`0`
                          (bind _state_19 (`self.AddDialogue` "A \"Heretic\"" "....... :')" (`|MakeArray` "Close" :!type "Text")))
                          (switch `/Game/Blueprints/Enum_DialogueState` _state_19
                            (:`NewEnumerator0`
                              (`self.ClearDialogueProgress`)
                              (`self.CloseConversation`)
                              (`self.SetDialogueTreeIndex` 3))))
                        (:`1`
                          (bind _state_20 (`self.AddDialogue` "A \"Heretic\"" "....... :'(" (`|MakeArray` "Close" :!type "Text")))
                          (switch `/Game/Blueprints/Enum_DialogueState` _state_20
                            (:`NewEnumerator0`
                              (`self.ClearDialogueProgress`)
                              (`self.CloseConversation`)
                              (`self.SetDialogueTreeIndex` 4))))))))))
            (:`1`
              (goto _label_2))
            (:`2`
              (goto _label_2))
            (:`3`
              (bind _state_21 (`self.AddDialogue` "A \"Heretic\"" ":')" (`|MakeArray` "Close" :!type "Text")))
              (switch `/Game/Blueprints/Enum_DialogueState` _state_21
                (:`NewEnumerator0`
                  (`self.ClearDialogueProgress`)
                  (`self.CloseConversation`))))
            (:`4`
              (bind _state_22 (`self.AddDialogue` "A \"Heretic\"" ":'(" (`|MakeArray` "Close" :!type "Text")))
              (switch `/Game/Blueprints/Enum_DialogueState` _state_22
                (:`NewEnumerator0`
                  (`self.ClearDialogueProgress`)
                  (`self.CloseConversation`))))))))))