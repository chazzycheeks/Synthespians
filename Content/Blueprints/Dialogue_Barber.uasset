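; Barber NPC dialogue Blueprint that overrides the parent Dialogue function to run a branching conversation about the district, the Architect and haircuts.
; When the ready-to-phone flag is set, only a player line about reporting in at the phone plays.
; Otherwise DialogueTreeIndex selects the first meeting, which sets the index to 1 on completion, or a shorter return chat.
; Chained AddDialogue calls branch on OptionIndex, with several paths rejoining shared lines.
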(fn `Dialogue`
  (`parent.Dialogue`)
  (bind _readytophone (`self.GetIsReadyToPhoneBool`))
  (if _readytophone
    (bind _state (`self.AddDialogue` "You" "I should report in at the phone." (`|MakeArray` "[Close]" :!type "Text")))
    (switch `/Game/Blueprints/Enum_DialogueState` _state
      (:`NewEnumerator0`
        (`self.ClearDialogueProgress`)
        (`self.CloseConversation`)))
    (else
      (switch `int` (`self.DialogueTreeIndex`)
        (:`0`
          (bind _state_2 (`self.AddDialogue` "Barber" "Pleasantries to you, Sir! Welcome, welcome." (`|MakeArray` "Hello" "Pleasantries" :!type "Text")))
          (switch `/Game/Blueprints/Enum_DialogueState` _state_2
            (:`NewEnumerator0`
              (bind (_state_3 _optionindex) (`self.AddDialogue` "Barber" "What can I help you with today?" (`|MakeArray` "How's your morning been?" "Where is everyone? The streets seem quiet" :!type "Text")))
              (switch `/Game/Blueprints/Enum_DialogueState` _state_3
                (:`NewEnumerator0`
                  (switch `int` _optionindex
                    (:`0`
                      (bind _state_4 (`self.AddDialogue` "Barber" "Fine thank you." (`|MakeArray` "[Next]" :!type "Text")))
                      (switch `/Game/Blueprints/Enum_DialogueState` _state_4
                        (:`NewEnumerator0`
                          (bind _state_5 (`self.AddDialogue` "Barber" "Yes, fine." (`|MakeArray` "[Next]" :!type "Text")))
                          (switch `/Game/Blueprints/Enum_DialogueState` _state_5
                            (:`NewEnumerator0`
                              (bind _state_6 (`self.AddDialogue` "Barber" "No trouble at all." (`|MakeArray` "[Next]" :!type "Text")))
                              (switch `/Game/Blueprints/Enum_DialogueState` _state_6
                                (:`NewEnumerator0`
                                  (bind _state_7 (`self.AddDialogue` "Barber" "Just the way we like it, hm?" (`|MakeArray` "Sure..." "Good to hear" :!type "Text")))
                                  (switch `/Game/Blueprints/Enum_DialogueState` _state_7
                                    (:`NewEnumerator0`
                                      (bind (_state_8 _optionindex_2) (`self.AddDialogue` "Barber" "Say friend, where are you from? I can tell it's not from around here." (`|MakeArray` "I'd appreciate if you kept that between us" "Is it that obvious?" :!type "Text") :!label _label))
                                      (switch `/Game/Blueprints/Enum_DialogueState` _state_8
                                        (:`NewEnumerator0`
                                          (switch `int` _optionindex_2
                                            (:`0`
                                              (bind _state_9 (`self.AddDialogue` "Barber" "Goodness, no, of course!" (`|MakeArray` "[Next]" :!type "Text")))
                                              (switch `/Game/Blueprints/Enum_DialogueState` _state_9
                                                (:`NewEnumerator0`
                                                  (bind _state_10 (`self.AddDialogue` "Barber" " It’s just… your hair. Very government." (`|MakeArray` "[Next]" :!type "Text")))
                                                  (switch `/Game/Blueprints/Enum_DialogueState` _state_10
                                                    (:`NewEnumerator0`
                                                      (bind _state_11 (`self.AddDialogue` "Barber" "Maybe you’d like a little help blending in?" (`|MakeArray` "Meaning what exactly?" "Such as?" :!type "Text")))
                                                      (switch `/Game/Blueprints/Enum_DialogueState` _state_11
                                                        (:`NewEnumerator0`
                                                          (bind _state_12 (`self.AddDialogue` "Barber" "A haircut, of course!" (`|MakeArray` "[Next]" :!type "Text")))
                                                          (switch `/Game/Blueprints/Enum_DialogueState` _state_12
                                                            (:`NewEnumerator0`
                                                              (bind _state_13 (`self.AddDialogue` "Barber" "We have four mighty fine options." (`|MakeArray` "[Next]" :!type "Text")))
                                                              (switch `/Game/Blueprints/Enum_DialogueState` _state_13
                                                                (:`NewEnumerator0`
                                                                  _)))))))))))
                                            (:`1`
                                              (bind _state_14 (`self.AddDialogue` "Barber" "Well... your haircut. Very government." (`|MakeArray` "[Next]" :!type "Text") :!label _label_2))
                                              (switch `/Game/Blueprints/Enum_DialogueState` _state_14
                                                (:`NewEnumerator0`
                                                  (bind (_state_15 _optionindex_3) (`self.AddDialogue` "Barber" "You see this district has a rather strict.." (`|MakeArray` "A strict what?" "I didn't realise it was any different" :!type "Text")))
                                                  (switch `/Game/Blueprints/Enum_DialogueState` _state_15
                                                    (:`NewEnumerator0`
                                                      (switch `int` _optionindex_3
                                                        (:`0`
                                                          (bind _state_16 (`self.AddDialogue` "Barber" "A- a strict standard of quality!" (`|MakeArray` "[Next]" :!type "Text")))
                                                          (switch `/Game/Blueprints/Enum_DialogueState` _state_16
                                                            (:`NewEnumerator0`
                                                              (bind _state_17 (`self.AddDialogue` "Barber" "Yes, that's right." (`|MakeArray` "[Next]" :!type "Text")))
                                                              (switch `/Game/Blueprints/Enum_DialogueState` _state_17
                                                                (:`NewEnumerator0`
                                                                  (bind _state_18 (`self.AddDialogue` "Barber" "Four excellent options, for men and women alike." (`|MakeArray` "[Next]" :!type "Text")))
                                                                  (switch `/Game/Blueprints/Enum_DialogueState` _state_18
                                                                    (:`NewEnumerator0`
                                                                      _)))))))
                                                        (:`1`
                                                          (bind _state_19 (`self.AddDialogue` "Barber" "Its subtle, yes - but we barbers are trained to notice." (`|MakeArray` "[Next]" :!type "Text")))
                                                          (switch `/Game/Blueprints/Enum_DialogueState` _state_19
                                                            (:`NewEnumerator0`
                                                              (bind _state_20 (`self.AddDialogue` "Barber" "There are four styles in this district. Each one… simply brilliant." (`|MakeArray` "[Next]" :!type "Text")))
                                                              (switch `/Game/Blueprints/Enum_DialogueState` _state_20
                                                                (:`NewEnumerator0`
                                                                  _)))))))))))))))))))))))
                    (:`1`
                      (bind _state_21 (`self.AddDialogue` "Barber" "Oh it's always like this." (`|MakeArray` "[Next]" :!type "Text")))
                      (switch `/Game/Blueprints/Enum_DialogueState` _state_21
                        (:`NewEnumerator0`
                          (bind (_state_22 _optionindex_4) (`self.AddDialogue` "Barber" "But you know what HE says - 'No reason to loiter when there's work to be done!'." (`|MakeArray` "I see..." "Right, of course" "Who is 'he'?" :!type "Text")))
                          (switch `/Game/Blueprints/Enum_DialogueState` _state_22
                            (:`NewEnumerator0`
                              (switch `int` _optionindex_4
                                (:`0`
                                  (goto _label))
                                (:`1`
                                  (goto _label))
                                (:`2`
                                  (bind _state_23 (`self.AddDialogue` "Barber" "The Archit...well its true, isn't it? Best to keep busy." (`|MakeArray` "[Next]" :!type "Text")))
                                  (switch `/Game/Blueprints/Enum_DialogueState` _state_23
                                    (:`NewEnumerator0`
                                      (bind (_state_24 _optionindex_5) (`self.AddDialogue` "Barber" "Especially we who have goverment positions." (`|MakeArray` "Right..." "'We'?" :!type "Text")))
                                      (switch `/Game/Blueprints/Enum_DialogueState` _state_24
                                        (:`NewEnumerator0`
                                          (switch `int` _optionindex_5
                                            (:`0`
                                              (goto _label))
                                            (:`1`
                                              (bind _state_25 (`self.AddDialogue` "Barber" "Oh I mean no disrespect, Sir! It's just.." (`|MakeArray` "Just what?" "Is it something I said?" :!type "Text")))
                                              (switch `/Game/Blueprints/Enum_DialogueState` _state_25
                                                (:`NewEnumerator0`
                                                  (goto _label_2)))))))))))))))))
                  (bind _state_26 (`self.AddDialogue` "Barber" "The Architect does encourage us to look our best." (`|MakeArray` "Only four?" "What are the options?" :!type "Text")))
                  (switch `/Game/Blueprints/Enum_DialogueState` _state_26
                    (:`NewEnumerator0`
                      (bind _state_27 (`self.AddDialogue` "Barber" "Two for men, two for women" (`|MakeArray` "[Next]" :!type "Text")))
                      (switch `/Game/Blueprints/Enum_DialogueState` _state_27
                        (:`NewEnumerator0`
                          (bind _state_28 (`self.AddDialogue` "Barber" "Unless you're State, of course. Then its a whole extra inch at the back!" (`|MakeArray` "[Next]" :!type "Text")))
                          (switch `/Game/Blueprints/Enum_DialogueState` _state_28
                            (:`NewEnumerator0`
                              (bind _state_29 (`self.AddDialogue` "Barber" "Of course... you’d know that I'm sure." (`|MakeArray` "[Next]" :!type "Text")))
                              (switch `/Game/Blueprints/Enum_DialogueState` _state_29
                                (:`NewEnumerator0`
                                  (bind _state_30 (`self.AddDialogue` "Barber" "Shall I bring you inside?" (`|MakeArray` "No, but thank you" "Another time" :!type "Text")))
                                  (switch `/Game/Blueprints/Enum_DialogueState` _state_30
                                    (:`NewEnumerator0`
                                      (bind _state_31 (`self.AddDialogue` "Barber" "Of course. Have a pleasant day, Sir..." (`|MakeArray` "[Next]" :!type "Text")))
                                      (switch `/Game/Blueprints/Enum_DialogueState` _state_31
                                        (:`NewEnumerator0`
                                          (bind _state_32 (`self.AddDialogue` "Barber" "Look after yourself." (`|MakeArray` "[Close]" :!type "Text")))
                                          (switch `/Game/Blueprints/Enum_DialogueState` _state_32
                                            (:`NewEnumerator0`
                                              (`self.SetDialogueTreeIndex` 1)
                                              (`self.ClearDialogueProgress`)
                                              (`self.CloseConversation`))))))))))))))))))))
        (:`1`
          (bind _state_33 (`self.AddDialogue` "Barber" "Pleasantries again to you Sir! " (`|MakeArray` "[Next]" :!type "Text")))
          (switch `/Game/Blueprints/Enum_DialogueState` _state_33
            (:`NewEnumerator0`
              (bind (_state_34 _optionindex_6) (`self.AddDialogue` "Barber" "Have you changed your mind about the haircut?" (`|MakeArray` "Can you remind me of my options?" "Actually I'm okay, thank you" :!type "Text")))
              (switch `/Game/Blueprints/Enum_DialogueState` _state_34
                (:`NewEnumerator0`
                  (switch `int` _optionindex_6
                    (:`0`
                      (bind _state_35 (`self.AddDialogue` "Barber" "Of course sir! You have two options, summer and winter." (`|MakeArray` "[Next]" :!type "Text")))
                      (switch `/Game/Blueprints/Enum_DialogueState` _state_35
                        (:`NewEnumerator0`
                          (bind _state_36 (`self.AddDialogue` "Barber" "Given it is fast approaching Autumn, I reccommend getting your Winter look in early!" (`|MakeArray` "[Next]" :!type "Text")))
                          (switch `/Game/Blueprints/Enum_DialogueState` _state_36
                            (:`NewEnumerator0`
                              (bind _state_37 (`self.AddDialogue` "Barber" "And of course you, my friend, get the extra inch!" (`|MakeArray` "[Next]" :!type "Text")))
                              (switch `/Game/Blueprints/Enum_DialogueState` _state_37
                                (:`NewEnumerator0`
                                  (bind (_state_38 _optionindex_7) (`self.AddDialogue` "Barber" "What do you say?" (`|MakeArray` "Nevermind, my apologies" "No thanks" :!type "Text")))
                                  (switch `/Game/Blueprints/Enum_DialogueState` _state_38
                                    (:`NewEnumerator0`
                                      (switch `int` _optionindex_7
                                        (:`0`
                                          (bind _state_39 (`self.AddDialogue` "Barber" "Not a problem Sir, have a pleasant day!" (`|MakeArray` "[Close]" :!type "Text")))
                                          (switch `/Game/Blueprints/Enum_DialogueState` _state_39
                                            (:`NewEnumerator0`
                                              (`self.ClearDialogueProgress`)
                                              (`self.CloseConversation`))))
                                        (:`1`
                                          (bind _state_40 (`self.AddDialogue` "Barber" "If you insist.." (`|MakeArray` "[Close]" :!type "Text")))
                                          (switch `/Game/Blueprints/Enum_DialogueState` _state_40
                                            (:`NewEnumerator0`
                                              (`self.ClearDialogueProgress`)
                                              (`self.CloseConversation`))))))))))))))
                    (:`1`
                      (bind _state_41 (`self.AddDialogue` "Barber" "No problem, have a most pleasant day." (`|MakeArray` "[Close]" :!type "Text")))
                      (switch `/Game/Blueprints/Enum_DialogueState` _state_41
                        (:`NewEnumerator0`
                          (`self.ClearDialogueProgress`)
                          (`self.CloseConversation`))))))))))))))