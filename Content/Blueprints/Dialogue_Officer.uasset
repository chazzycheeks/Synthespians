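; Dialogue script for the Officer NPC, a checkpoint guard who demands the player's papers, warns of Heretic activity and recognizes Directorate credentials.
; The Dialogue override calls its parent, then switches on DialogueTreeIndex between the first conversation and a shorter return conversation.
; Chained AddDialogue calls continue on Pass Through, branching on OptionIndex with shared reconvergence points.
; First-conversation endings set the tree index to 1, clear progress and close.
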(fn `Dialogue`
  (`parent.Dialogue`)
  (switch `int` (`self.DialogueTreeIndex`)
    (:`0`
      (bind _state (`self.AddDialogue` "Officer" "Pleasantries." (`|MakeArray` "Hello" "Pleasantries" :!type "Text")))
      (switch `/Game/Blueprints/Enum_DialogueState` _state
        (:`NewEnumerator0`
          (bind (_state_2 _optionindex) (`self.AddDialogue` "Officer" "I'll need to see your papers, please." (`|MakeArray` "I forgot them" "Why is that?" "I suppose" :!type "Text")))
          (switch `/Game/Blueprints/Enum_DialogueState` _state_2
            (:`NewEnumerator0`
              (switch `int` _optionindex
                (:`0`
                  (bind (_state_3 _optionindex_2) (`self.AddDialogue` "Officer" "No papers, no travel. Simple as that I’m afraid." (`|MakeArray` "You run a tight ship" "Right... here you are then…" :!type "Text")))
                  (switch `/Game/Blueprints/Enum_DialogueState` _state_3
                    (:`NewEnumerator0`
                      (switch `int` _optionindex_2
                        (:`0`
                          (bind (_state_4 _optionindex_3) (`self.AddDialogue` "Officer" "Haven’t got a choice… Heretic activity is on the rise in this district. No room for complacency. " (`|MakeArray` "What kind of activity?" "These Heretics… what do you know about them?" :!type "Text")))
                          (switch `/Game/Blueprints/Enum_DialogueState` _state_4
                            (:`NewEnumerator0`
                              (switch `int` _optionindex_3 :!label _label
                                (:`0`
                                  (bind _state_5 (`self.AddDialogue` "Officer" "They're spreading ideas... Dangerous ones." (`|MakeArray` "[Next]" :!type "Text")))
                                  (switch `/Game/Blueprints/Enum_DialogueState` _state_5
                                    (:`NewEnumerator0`
                                      (bind _state_6 (`self.AddDialogue` "Officer" "The kind that make good people start asking questions.." (`|MakeArray` "I see.." "I best be going.." :!type "Text")))
                                      (switch `/Game/Blueprints/Enum_DialogueState` _state_6
                                        (:`NewEnumerator0`
                                          (bind _state_7 (`self.AddDialogue` "Officer" "The kind that make good people start asking questions.." (`|MakeArray` "I see.." "I best be going.." :!type "Text")))
                                          (switch `/Game/Blueprints/Enum_DialogueState` _state_7
                                            (:`NewEnumerator0`
                                              _)))))))
                                (:`1`
                                  (bind _state_8 (`self.AddDialogue` "Officer" "Not much to know. They blend in. Smile like the rest of us." (`|MakeArray` "[Next]" :!type "Text")))
                                  (switch `/Game/Blueprints/Enum_DialogueState` _state_8
                                    (:`NewEnumerator0`
                                      (bind _state_9 (`self.AddDialogue` "Officer" "But sooner or later, they slip up… That’s when you report them. Fast." (`|MakeArray` "You've been very helpful" "Good speaking with you" :!type "Text")))
                                      (switch `/Game/Blueprints/Enum_DialogueState` _state_9
                                        (:`NewEnumerator0`
                                          _))))))
                              (bind _state_10 (`self.AddDialogue` "Officer" "You have a pleasant day now." (`|MakeArray` "[Close]" :!type "Text")))
                              (switch `/Game/Blueprints/Enum_DialogueState` _state_10
                                (:`NewEnumerator0`
                                  (`self.SetDialogueTreeIndex` 1)
                                  (`self.ClearDialogueProgress`)
                                  (`self.CloseConversation`))))))
                        (:`1`
                          (bind (_state_11 _optionindex_4) (`self.AddDialogue` "Officer" "Oh! Directorate credentials. So you’re the one they’ve sent?" (`|MakeArray` "Something like that" "I think you must be mistaken" :!type "Text") :!label _label_2))
                          (switch `/Game/Blueprints/Enum_DialogueState` _state_11
                            (:`NewEnumerator0`
                              (switch `int` _optionindex_4
                                (:`0`
                                  (bind (_state_12 _optionindex_5) (`self.AddDialogue` "Officer" "Have you found any traitors yet?" (`|MakeArray` "Still working on it" "Don't suppose you have any tips?" :!type "Text")))
                                  (switch `/Game/Blueprints/Enum_DialogueState` _state_12
                                    (:`NewEnumerator0`
                                      (switch `int` _optionindex_5
                                        (:`0`
                                          (bind _state_13 (`self.AddDialogue` "Officer" "Well don’t waste any time. " (`|MakeArray` "[Next]" :!type "Text")))
                                          (switch `/Game/Blueprints/Enum_DialogueState` _state_13
                                            (:`NewEnumerator0`
                                              (bind _state_14 (`self.AddDialogue` "Officer" "These people are everywhere, you know… smiling, nodding, pretending to fit in. " (`|MakeArray` "[Next]" :!type "Text")))
                                              (switch `/Game/Blueprints/Enum_DialogueState` _state_14
                                                (:`NewEnumerator0`
                                                  (bind _state_15 (`self.AddDialogue` "Officer" " The State has no use for those wishing to rewrite The Architect's hard work." (`|MakeArray` "You've been very helpful" "Good speaking with you" :!type "Text")))
                                                  (switch `/Game/Blueprints/Enum_DialogueState` _state_15
                                                    (:`NewEnumerator0`
                                                      _)))))))
                                        (:`1`
                                          (bind _state_16 (`self.AddDialogue` "Officer" "Hmm. Between us, there’s been talk about the shops on Main. Some of the owners have been… unsettled lately." (`|MakeArray` "[Next]" :!type "Text")))
                                          (switch `/Game/Blueprints/Enum_DialogueState` _state_16
                                            (:`NewEnumerator0`
                                              (bind _state_17 (`self.AddDialogue` "Officer" "Just remember, don’t let sympathy cloud your purpose." (`|MakeArray` "[Next]" :!type "Text")))
                                              (switch `/Game/Blueprints/Enum_DialogueState` _state_17
                                                (:`NewEnumerator0`
                                                  (bind _state_18 (`self.AddDialogue` "Officer" "These people reject the very system that keeps us alive. The State has no use for them. " (`|MakeArray` "Sure.." "Not to worry" :!type "Text")))
                                                  (switch `/Game/Blueprints/Enum_DialogueState` _state_18
                                                    (:`NewEnumerator0`
                                                      (bind _state_19 (`self.AddDialogue` "Officer" "Excellent." (`|MakeArray` "[Next]" :!type "Text")))
                                                      (switch `/Game/Blueprints/Enum_DialogueState` _state_19
                                                        (:`NewEnumerator0`
                                                          _))))))))))
                                      (bind _state_20 (`self.AddDialogue` "Officer" "You have a pleasant day now, Sir. Good luck..." (`|MakeArray` "[Close]" :!type "Text")))
                                      (switch `/Game/Blueprints/Enum_DialogueState` _state_20
                                        (:`NewEnumerator0`
                                          (`self.SetDialogueTreeIndex` 1)
                                          (`self.ClearDialogueProgress`)
                                          (`self.CloseConversation`))))))
                                (:`1`
                                  (bind _state_21 (`self.AddDialogue` "Officer" "Look, the street border’s closed until further notice. Increase of Heretic activity." (`|MakeArray` "[Next]" :!type "Text") :!label _label_3))
                                  (switch `/Game/Blueprints/Enum_DialogueState` _state_21
                                    (:`NewEnumerator0`
                                      (bind _state_22 (`self.AddDialogue` "Officer" "No comings or goings until they wave the order." (`|MakeArray` "What kind of activity?" "These Heretics… what do you know about them?" :!type "Text")))
                                      (switch `/Game/Blueprints/Enum_DialogueState` _state_22
                                        (:`NewEnumerator0`
                                          (goto _label))))))))))))))
                (:`1`
                  (bind (_state_23 _optionindex_6) (`self.AddDialogue` "Officer" " Just a quick formality, I’m sure you understand.." (`|MakeArray` "Of course" "Seems like I don't have a choice" :!type "Text") :!label _label_4))
                  (switch `/Game/Blueprints/Enum_DialogueState` _state_23
                    (:`NewEnumerator0`
                      (switch `int` _optionindex_6
                        (:`0`
                          (goto _label_2))
                        (:`1`
                          (bind (_state_24 _optionindex_7) (`self.AddDialogue` "Officer" "That kind of speak won’t get you very far around here, Sir. Not far at all." (`|MakeArray` "It's got me here hasn't it" "Apologies officer" :!type "Text")))
                          (switch `/Game/Blueprints/Enum_DialogueState` _state_24
                            (:`NewEnumerator0`
                              (switch `int` _optionindex_7
                                (:`0`
                                  (bind _state_25 (`self.AddDialogue` "Officer" " Do. Not. Test. Me" (`|MakeArray` "Ok then" "My apologies" :!type "Text")))
                                  (switch `/Game/Blueprints/Enum_DialogueState` _state_25
                                    (:`NewEnumerator0`
                                      (goto _label_3))))
                                (:`1`
                                  (goto _label_3))))))))))
                (:`2`
                  (goto _label_4))))))))
    (:`1`
      (bind (_state_26 _optionindex_8) (`self.AddDialogue` "Officer" "Pleasanties, was there something else?" (`|MakeArray` "Any more info on spotting a Heretic?" "No, nevermind" :!type "Text")))
      (switch `/Game/Blueprints/Enum_DialogueState` _state_26
        (:`NewEnumerator0`
          (switch `int` _optionindex_8
            (:`0`
              (bind _state_27 (`self.AddDialogue` "Officer" "Looks can be decieving, they could be any one of us. " (`|MakeArray` "[Next]" :!type "Text")))
              (switch `/Game/Blueprints/Enum_DialogueState` _state_27
                (:`NewEnumerator0`
                  (bind _state_28 (`self.AddDialogue` "Officer" "That is what what makes them so dangerous." (`|MakeArray` "[Next]" :!type "Text")))
                  (switch `/Game/Blueprints/Enum_DialogueState` _state_28
                    (:`NewEnumerator0`
                      (bind _state_29 (`self.AddDialogue` "Officer" "Be careful, and remain vigilant." (`|MakeArray` "[Close]" :!type "Text")))
                      (switch `/Game/Blueprints/Enum_DialogueState` _state_29
                        (:`NewEnumerator0`
                          (`self.ClearDialogueProgress`)
                          (`self.CloseConversation`))))))))
            (:`1`
              (`self.ClearDialogueProgress`)
              (`self.CloseConversation`))))))))