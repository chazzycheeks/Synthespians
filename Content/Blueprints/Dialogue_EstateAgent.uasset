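; Branching dialogue for the Travel Agent NPC, who can be drawn into confiding forbidden wishes to cross the border.
; Overrides Dialogue, gating on the ready-to-phone flag, then picking conversations by level progress, tree index and whether they have spoken.
; Nested AddDialogue calls advance on Pass Through and branch on option index, with shared labels merging paths.
; The confession posts a Lightbulb Wwise event, advances level progress and rings the phone box.
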(fn `Dialogue`
  (`parent.Dialogue`)
  (bind _readytophone (`self.GetIsReadyToPhoneBool`))
  (if _readytophone
    (bind _state (`self.AddDialogue` "You" "I should report in at the phone." (`|MakeArray` "[Close]" :!type "Text")))
    (switch `/Game/Blueprints/Enum_DialogueState` _state
      (:`NewEnumerator0`
        (`self.ClearDialogueProgress`)
        (`self.CloseConversation`)))
    (else
      (bind _this_index (`self.GetLevelProgressIndex`))
      (switch `int` _this_index
        (:`0`
          (switch `int` (`self.DialogueTreeIndex`)
            (:`0`
              (bind _state_2 (`self.AddDialogue` "Travel Agent" "..." (`|MakeArray` "Hello" "Pleasantries" :!type "Text")))
              (switch `/Game/Blueprints/Enum_DialogueState` _state_2
                (:`NewEnumerator0`
                  (bind _state_3 (`self.AddDialogue` "Travel Agent" "Oh- Pleasantries to you, friend!" (`|MakeArray` "[Next]" :!type "Text")))
                  (switch `/Game/Blueprints/Enum_DialogueState` _state_3
                    (:`NewEnumerator0`
                      (bind _state_4 (`self.AddDialogue` "Travel Agent" "I’m afraid the Travel Agency’s closed at the minute." (`|MakeArray` "That's alright" "Ah, shame, was hoping for a chat" :!type "Text")))
                      (switch `/Game/Blueprints/Enum_DialogueState` _state_4
                        (:`NewEnumerator0`
                          (bind _state_5 (`self.AddDialogue` "Travel Agent" "Do find me later on, conversation is a real luxury these days. " (`|MakeArray` "[Next]" :!type "Text")))
                          (switch `/Game/Blueprints/Enum_DialogueState` _state_5
                            (:`NewEnumerator0`
                              (bind _state_6 (`self.AddDialogue` "Travel Agent" "Pleasant day!" (`|MakeArray` "[Close]" :!type "Text")))
                              (switch `/Game/Blueprints/Enum_DialogueState` _state_6
                                (:`NewEnumerator0`
                                  (`self.SetDialogueTreeIndex` 1)
                                  (set `self.HaveSpoken` true)
                                  (`self.ClearDialogueProgress`)
                                  (`self.CloseConversation`))))))))))))
            (:`1`
              (bind _state_7 (`self.AddDialogue` "Travel Agent" "Apologies friend! Let's talk another time." (`|MakeArray` "[Close]" :!type "Text")))
              (switch `/Game/Blueprints/Enum_DialogueState` _state_7
                (:`NewEnumerator0`
                  (`self.ClearDialogueProgress`)
                  (`self.CloseConversation`))))))
        (:`1`
          (switch `int` (`self.DialogueTreeIndex`)
            (:`0`
              (if (`self.HaveSpoken`) :!label _label
                (bind (_state_8 _optionindex) (`self.AddDialogue` "Travel Agent" "Ah! Pleasantries agan to you, Sir! Apologies for yesterday, how can I help you?" (`|MakeArray` "Just getting my bearings" "New to the area,  thought I'd pop by" :!type "Text")))
                (switch `/Game/Blueprints/Enum_DialogueState` _state_8
                  (:`NewEnumerator0`
                    (switch `int` _optionindex
                      (:`0`
                        (bind _state_9 (`self.AddDialogue` "Travel Agent" "Indeed, as am I! I'm a countryside man myself." (`|MakeArray` "[Next]" :!type "Text") :!label _label_2))
                        (switch `/Game/Blueprints/Enum_DialogueState` _state_9
                          (:`NewEnumerator0`
                            (bind _state_10 (`self.AddDialogue` "Travel Agent" "B-but I love this city, of course- Yes!" (`|MakeArray` "Strange place to end up" "What brought you to this sector?" :!type "Text") :!label _label_3))
                            (switch `/Game/Blueprints/Enum_DialogueState` _state_10
                              (:`NewEnumerator0`
                                (bind _state_11 (`self.AddDialogue` "Travel Agent" "That’d be the work-service program. Name was drawn and here’s where it sent me." (`|MakeArray` "[Next]" :!type "Text")))
                                (switch `/Game/Blueprints/Enum_DialogueState` _state_11
                                  (:`NewEnumerator0`
                                    (bind (_state_12 _optionindex_2) (`self.AddDialogue` "Travel Agent" "It's an...efficient system, I suppose. I know the boondocks well you see! I assume that's why I was chosen." (`|MakeArray` "Do you get home much?" "They can just relocate you like that?" :!type "Text")))
                                    (switch `/Game/Blueprints/Enum_DialogueState` _state_12
                                      (:`NewEnumerator0`
                                        (switch `int` _optionindex_2
                                          (:`0`
                                            (bind (_state_13 _optionindex_3) (`self.AddDialogue` "Travel Agent" " Home... Goodness, no. Can't imagine I’d get approval." (`|MakeArray` "Perhaps the State is wrong for that" "Seems cruel" "Yeah fair enough" :!type "Text")))
                                            (switch `/Game/Blueprints/Enum_DialogueState` _state_13
                                              (:`NewEnumerator0`
                                                (switch `int` _optionindex_3
                                                  (:`0`
                                                    (bind _state_14 (`self.AddDialogue` "Travel Agent" "-No! It's fine." (`|MakeArray` "[Next]" :!type "Text") :!label _label_4))
                                                    (switch `/Game/Blueprints/Enum_DialogueState` _state_14
                                                      (:`NewEnumerator0`
                                                        (bind _state_15 (`self.AddDialogue` "Travel Agent" "More than fine. I'm blessed to be here." (`|MakeArray` "[Next]" :!type "Text")))
                                                        (switch `/Game/Blueprints/Enum_DialogueState` _state_15
                                                          (:`NewEnumerator0`
                                                            (bind _state_16 (`self.AddDialogue` "Travel Agent" "You have a pleasant day now, Sir, I should get to work... " (`|MakeArray` "[Close]" :!type "Text")))
                                                            (switch `/Game/Blueprints/Enum_DialogueState` _state_16
                                                              (:`NewEnumerator0`
                                                                (`self.SetDialogueTreeIndex` 2)
                                                                (`self.ClearDialogueProgress`)
                                                                (`self.CloseConversation`))))))))
                                                  (:`1`
                                                    (goto _label_4))
                                                  (:`2`
                                                    (bind _state_17 (`self.AddDialogue` "Travel Agent" "..." (`|MakeArray` "[Next]" :!type "Text") :!label _label_5))
                                                    (switch `/Game/Blueprints/Enum_DialogueState` _state_17
                                                      (:`NewEnumerator0`
                                                        (bind _state_18 (`self.AddDialogue` "Travel Agent" "Can- can I interest you in any package holidays Sir?! We’ve got an excellent selection. " (`|MakeArray` "[Next]" :!type "Text")))
                                                        (switch `/Game/Blueprints/Enum_DialogueState` _state_18
                                                          (:`NewEnumerator0`
                                                            (bind (_state_19 _optionindex_4) (`self.AddDialogue` "Travel Agent" "Everything you could ever want to see, right here on home ground." (`|MakeArray` "Sounds like you're reading a script" "State sponsored is it?" :!type "Text")))
                                                            (switch `/Game/Blueprints/Enum_DialogueState` _state_19
                                                              (:`NewEnumerator0`
                                                                (switch `int` _optionindex_4
                                                                  (:`0`
                                                                    (bind (_state_20 _optionindex_5) (`self.AddDialogue` "Travel Agent" "Ha- well...you know how it goes around here." (`|MakeArray` "You must want to see other places...out of State?" "Speaking fluent propaganda" :!type "Text") :!label _label_6))
                                                                    (switch `/Game/Blueprints/Enum_DialogueState` _state_20
                                                                      (:`NewEnumerator0`
                                                                        (switch `int` _optionindex_5
                                                                          (:`0`
                                                                            (bind _state_21 (`self.AddDialogue` "Travel Agent" "...Of course, but- please, don’t ask me that." (`|MakeArray` "[Next]" :!type "Text") :!label _label_7))
                                                                            (switch `/Game/Blueprints/Enum_DialogueState` _state_21
                                                                              (:`NewEnumerator0`
                                                                                (bind _state_22 (`self.AddDialogue` "Travel Agent" "Sorry." (`|MakeArray` "[Next]" :!type "Text")))
                                                                                (switch `/Game/Blueprints/Enum_DialogueState` _state_22
                                                                                  (:`NewEnumerator0`
                                                                                    (bind (_state_23 _optionindex_6) (`self.AddDialogue` "Travel Agent" "It’s not a safe sort of question, you understand?" (`|MakeArray` "You can trust me, promise" "It wont leave this conversation" "You're right, I'm sorry" :!type "Text")))
                                                                                    (switch `/Game/Blueprints/Enum_DialogueState` _state_23
                                                                                      (:`NewEnumerator0`
                                                                                        (switch `int` _optionindex_6
                                                                                          (:`0`
                                                                                            (bind _state_24 (`self.AddDialogue` "Travel Agent" "Okay...If you must know..." (`|MakeArray` "[Next]" :!type "Text") :!label _label_8))
                                                                                            (switch `/Game/Blueprints/Enum_DialogueState` _state_24
                                                                                              (:`NewEnumerator0`
                                                                                                (bind _state_25 (`self.AddDialogue` "Travel Agent" "I’d visit my family." (`|MakeArray` "[Next]" :!type "Text")))
                                                                                                (switch `/Game/Blueprints/Enum_DialogueState` _state_25
                                                                                                  (:`NewEnumerator0`
                                                                                                    (bind _state_26 (`self.AddDialogue` "Travel Agent" "My extended family, just across the border in a tiny village." (`|MakeArray` "[Next]" :!type "Text")))
                                                                                                    (switch `/Game/Blueprints/Enum_DialogueState` _state_26
                                                                                                      (:`NewEnumerator0`
                                                                                                        (bind _state_27 (`self.AddDialogue` "Travel Agent" "Before my father passed, he used to tell me stories about them. " (`|MakeArray` "[Next]" :!type "Text")))
                                                                                                        (switch `/Game/Blueprints/Enum_DialogueState` _state_27
                                                                                                          (:`NewEnumerator0`
                                                                                                            (bind _state_28 (`self.AddDialogue` "Travel Agent" "Old stories now about cousins, uncles… People I’ve never met. " (`|MakeArray` "[Next]" :!type "Text")))
                                                                                                            (switch `/Game/Blueprints/Enum_DialogueState` _state_28
                                                                                                              (:`NewEnumerator0`
                                                                                                                (bind _state_29 (`self.AddDialogue` "Travel Agent" "To think- my own kin, living their lives barely a hundred miles south of here, and we’ve never once met. " (`|MakeArray` "[Next]" :!type "Text")))
                                                                                                                (switch `/Game/Blueprints/Enum_DialogueState` _state_29
                                                                                                                  (:`NewEnumerator0`
                                                                                                                    (bind (_state_30 _optionindex_7) (`self.AddDialogue` "Travel Agent" "I know it’s not Rome or Tokyo, or at least what you hear about them... but to me, its more important than anything else. That’s where I’d go. " (`|MakeArray` "That's a beautiful dream" "Have you ever considered...crossing over?" :!type "Text")))
                                                                                                                    (switch `/Game/Blueprints/Enum_DialogueState` _state_30
                                                                                                                      (:`NewEnumerator0`
                                                                                                                        (switch `int` _optionindex_7
                                                                                                                          (:`0`
                                                                                                                            (bind _state_31 (`self.AddDialogue` "Travel Agent" "We knew things were getting bad when the airports shut. " (`|MakeArray` "[Next]" :!type "Text")))
                                                                                                                            (switch `/Game/Blueprints/Enum_DialogueState` _state_31
                                                                                                                              (:`NewEnumerator0`
                                                                                                                                (bind _state_32 (`self.AddDialogue` "Travel Agent" "Then there was the roads- blockaded over night. " (`|MakeArray` "[Next]" :!type "Text")))
                                                                                                                                (switch `/Game/Blueprints/Enum_DialogueState` _state_32
                                                                                                                                  (:`NewEnumerator0`
                                                                                                                                    (bind _state_33 (`self.AddDialogue` "Travel Agent" "They said it was to keep our enemies out..." (`|MakeArray` "[Next]" :!type "Text")))
                                                                                                                                    (switch `/Game/Blueprints/Enum_DialogueState` _state_33
                                                                                                                                      (:`NewEnumerator0`
                                                                                                                                        (bind _state_34 (`self.AddDialogue` "Travel Agent" "..but look at us now. \"Thank the Architect\"... Bollocks. " (`|MakeArray` "[Next]" :!type "Text")))
                                                                                                                                        (switch `/Game/Blueprints/Enum_DialogueState` _state_34
                                                                                                                                          (:`NewEnumerator0`
                                                                                                                                            _)))))))))
                                                                                                                          (:`1`
                                                                                                                            (bind _state_35 (`self.AddDialogue` "Travel Agent" "Golly, of course- but I haven’t dared. Some are trying, though." (`|MakeArray` "[Next]" :!type "Text")))
                                                                                                                            (switch `/Game/Blueprints/Enum_DialogueState` _state_35
                                                                                                                              (:`NewEnumerator0`
                                                                                                                                (bind _state_36 (`self.AddDialogue` "Travel Agent" "Hand-drawn maps, passed round in secret.." (`|MakeArray` "[Next]" :!type "Text")))
                                                                                                                                (switch `/Game/Blueprints/Enum_DialogueState` _state_36
                                                                                                                                  (:`NewEnumerator0`
                                                                                                                                    (bind _state_37 (`self.AddDialogue` "Travel Agent" " I- I bought one... " (`|MakeArray` "[Next]" :!type "Text")))
                                                                                                                                    (switch `/Game/Blueprints/Enum_DialogueState` _state_37
                                                                                                                                      (:`NewEnumerator0`
                                                                                                                                        _))))))))
                                                                                                                        (bind _state_38 (`self.AddDialogue` "Travel Agent" "Sorry-I've said far too much... I’ll need to be on my way now Sir. " (`|MakeArray` "[Next]" :!type "Text")))
                                                                                                                        (switch `/Game/Blueprints/Enum_DialogueState` _state_38
                                                                                                                          (:`NewEnumerator0`
                                                                                                                            (`AkGameplayStatics.PostEvent` "/Game/WwiseAudio/Events/MUSIC/Lightbulb.Lightbulb")
                                                                                                                            (bind (_state_39 _optionindex_8) (`self.AddDialogue` "Travel Agent" "I trust you won't speak of this to anyone?" (`|MakeArray` "Of course" "Well..." "Don't you trust me?" :!type "Text")))
                                                                                                                            (switch `/Game/Blueprints/Enum_DialogueState` _state_39
                                                                                                                              (:`NewEnumerator0`
                                                                                                                                (switch `int` _optionindex_8
                                                                                                                                  (:`0`
                                                                                                                                    (bind _state_40 (`self.AddDialogue` "Travel Agent" "Good good. Sorry, you can't be too careful. Take care now." (`|MakeArray` "[Close]" :!type "Text")))
                                                                                                                                    (switch `/Game/Blueprints/Enum_DialogueState` _state_40
                                                                                                                                      (:`NewEnumerator0`
                                                                                                                                        _)))
                                                                                                                                  (:`1`
                                                                                                                                    (bind _state_41 (`self.AddDialogue` "Travel Agent" ".......Goodbye." (`|MakeArray` "[Close]" :!type "Text")))
                                                                                                                                    (switch `/Game/Blueprints/Enum_DialogueState` _state_41
                                                                                                                                      (:`NewEnumerator0`
                                                                                                                                        _)))
                                                                                                                                  (:`2`
                                                                                                                                    (bind _state_42 (`self.AddDialogue` "Travel Agent" "No no of course friend! I just needed to confirm, for my own sake, I'm sure you understand. " (`|MakeArray` "[Next]" :!type "Text")))
                                                                                                                                    (switch `/Game/Blueprints/Enum_DialogueState` _state_42
                                                                                                                                      (:`NewEnumerator0`
                                                                                                                                        (bind _state_43 (`self.AddDialogue` "Travel Agent" "I really should go now. Look after yourself." (`|MakeArray` "[Close]" :!type "Text")))
                                                                                                                                        (switch `/Game/Blueprints/Enum_DialogueState` _state_43
                                                                                                                                          (:`NewEnumerator0`
                                                                                                                                            _))))))
                                                                                                                                (`self.SetLevelProgressIndex` 2)
                                                                                                                                (`self.SetIsReadyToPhoneBool` true)
                                                                                                                                (`self.ClearDialogueProgress`)
                                                                                                                                (`self.CloseConversation`)
                                                                                                                                (bind _returnvalue (`GameplayStatics.GetActorOfClass` "/Game/Models/BP_Phonebox.BP_Phonebox_C"))
                                                                                                                                (`/Game/Models/BP_Phonebox.ringing` _returnvalue))))))))))))))))))))
                                                                                          (:`1`
                                                                                            (goto _label_8))
                                                                                          (:`2`
                                                                                            (bind _state_44 (`self.AddDialogue` "Travel Agent" "Yes... Not safe...I should get going." (`|MakeArray` "[Next]" :!type "Text")))
                                                                                            (switch `/Game/Blueprints/Enum_DialogueState` _state_44
                                                                                              (:`NewEnumerator0`
                                                                                                (bind _state_45 (`self.AddDialogue` "Travel Agent" "Speak soon perhaps..." (`|MakeArray` "[Close]" :!type "Text")))
                                                                                                (switch `/Game/Blueprints/Enum_DialogueState` _state_45
                                                                                                  (:`NewEnumerator0`
                                                                                                    (`self.SetDialogueTreeIndex` 3)
                                                                                                    (`self.ClearDialogueProgress`)
                                                                                                    (`self.CloseConversation`))))))))))))))
                                                                          (:`1`
                                                                            (bind _state_46 (`self.AddDialogue` "Travel Agent" "Eheh... I- I’ll need to be going now Sir. Very busy." (`|MakeArray` "[Next]" :!type "Text")))
                                                                            (switch `/Game/Blueprints/Enum_DialogueState` _state_46
                                                                              (:`NewEnumerator0`
                                                                                (bind _state_47 (`self.AddDialogue` "Travel Agent" "You have yourself a pleasant day now." (`|MakeArray` "[Close]" :!type "Text")))
                                                                                (switch `/Game/Blueprints/Enum_DialogueState` _state_47
                                                                                  (:`NewEnumerator0`
                                                                                    (`self.SetDialogueTreeIndex` 2)
                                                                                    (`self.ClearDialogueProgress`)
                                                                                    (`self.CloseConversation`))))))))))
                                                                  (:`1`
                                                                    (bind _state_48 (`self.AddDialogue` "Travel Agent" "Part of the improved Domestic Discovery Initiative. " (`|MakeArray` "[Next]" :!type "Text") :!label _label_9))
                                                                    (switch `/Game/Blueprints/Enum_DialogueState` _state_48
                                                                      (:`NewEnumerator0`
                                                                        (bind _state_49 (`self.AddDialogue` "Travel Agent" "Marvellous program… It supports local tourism." (`|MakeArray` "[Next]" :!type "Text")))
                                                                        (switch `/Game/Blueprints/Enum_DialogueState` _state_49
                                                                          (:`NewEnumerator0`
                                                                            (bind _state_50 (`self.AddDialogue` "Travel Agent" "Keeps the economy strong, and people- well, tightly packed together." (`|MakeArray` "Sure, but don't you want to go elsewhere?" "You ever get the urge to visit a different country?" :!type "Text")))
                                                                            (switch `/Game/Blueprints/Enum_DialogueState` _state_50
                                                                              (:`NewEnumerator0`
                                                                                (goto _label_7))))))))))))))))))))
                                          (:`1`
                                            (goto _label_5))))))))))))
                      (:`1`
                        (bind _state_51 (`self.AddDialogue` "Travel Agent" "Ah, well, I’m sure you’ll settle in no time! " (`|MakeArray` "[Next]" :!type "Text") :!label _label_10))
                        (switch `/Game/Blueprints/Enum_DialogueState` _state_51
                          (:`NewEnumerator0`
                            (bind (_state_52 _optionindex_9) (`self.AddDialogue` "Travel Agent" "Bit quiet at first, but that’s part of the charm. You get used to it…everyone does" (`|MakeArray` "Quiet suits me, actually" "What trips are you selling?" :!type "Text")))
                            (switch `/Game/Blueprints/Enum_DialogueState` _state_52
                              (:`NewEnumerator0`
                                (switch `int` _optionindex_9
                                  (:`0`
                                    (bind _state_53 (`self.AddDialogue` "Travel Agent" "Me too! I'm a countryside man myself." (`|MakeArray` "[Next]" :!type "Text")))
                                    (switch `/Game/Blueprints/Enum_DialogueState` _state_53
                                      (:`NewEnumerator0`
                                        (goto _label_3))))
                                  (:`1`
                                    (bind _state_54 (`self.AddDialogue` "Travel Agent" "Well we do all sorts here! Tours, bookings, local recommendations. All Architect approved!" (`|MakeArray` "[Next]" :!type "Text")))
                                    (switch `/Game/Blueprints/Enum_DialogueState` _state_54
                                      (:`NewEnumerator0`
                                        (bind _state_55 (`self.AddDialogue` "Travel Agent" "You’d be amazed at what’s right on your doorstep." (`|MakeArray` "Local spots?" "You mean day trips?" :!type "Text")))
                                        (switch `/Game/Blueprints/Enum_DialogueState` _state_55
                                          (:`NewEnumerator0`
                                            (bind _state_56 (`self.AddDialogue` "Travel Agent" "Precisely. Say- if you’re looking for something restorative, the lakes out east are just excellent. " (`|MakeArray` "[Next]" :!type "Text")))
                                            (switch `/Game/Blueprints/Enum_DialogueState` _state_56
                                              (:`NewEnumerator0`
                                                (bind _state_57 (`self.AddDialogue` "Travel Agent" "Crystal waters, clean air - people say it feels like another world." (`|MakeArray` "Sounds like paradise" "Impressive" "Another world, huh?" :!type "Text")))
                                                (switch `/Game/Blueprints/Enum_DialogueState` _state_57
                                                  (:`NewEnumerator0`
                                                    (bind _state_58 (`self.AddDialogue` "Travel Agent" "We used to think flying was the only way to find wonder.  But truly, everything worth seeing is right here. " (`|MakeArray` "[Next]" :!type "Text")))
                                                    (switch `/Game/Blueprints/Enum_DialogueState` _state_58
                                                      (:`NewEnumerator0`
                                                        (bind (_state_59 _optionindex_10) (`self.AddDialogue` "Travel Agent" "The forests, the hills, the markets.. We’ve certainly come to appreciate what’s ours." (`|MakeArray` "Sounds like you're reading a script" "State sponsored is it?" :!type "Text")))
                                                        (switch `/Game/Blueprints/Enum_DialogueState` _state_59
                                                          (:`NewEnumerator0`
                                                            (switch `int` _optionindex_10
                                                              (:`0`
                                                                (goto _label_6))
                                                              (:`1`
                                                                (goto _label_9)))))))))))))))))))))))))
                (else
                  (bind (_state_60 _optionindex_11) (`self.AddDialogue` "Travel Agent" "Pleasantries, Sir! How can I help?" (`|MakeArray` "Just getting my bearings" "New to the area,  thought I'd pop by" :!type "Text")))
                  (switch `/Game/Blueprints/Enum_DialogueState` _state_60
                    (:`NewEnumerator0`
                      (switch `int` _optionindex_11
                        (:`0`
                          (goto _label_2))
                        (:`1`
                          (goto _label_10))))))))
            (:`1`
              (goto _label))
            (:`2`
              (bind (_state_61 _optionindex_12) (`self.AddDialogue` "Travel Agent" "...Was there something else you needed?" (`|MakeArray` "Nevermind, sorry" "Can I ask about any State programs you have?" :!type "Text")))
              (switch `/Game/Blueprints/Enum_DialogueState` _state_61
                (:`NewEnumerator0`
                  (switch `int` _optionindex_12
                    (:`0`
                      (`self.ClearDialogueProgress`)
                      (`self.CloseConversation`))
                    (:`1`
                      (bind _state_62 (`self.AddDialogue` "Travel Agent" "Y-yes of course, Sir!" (`|MakeArray` "[Next]" :!type "Text")))
                      (switch `/Game/Blueprints/Enum_DialogueState` _state_62
                        (:`NewEnumerator0`
                          (bind _state_63 (`self.AddDialogue` "Travel Agent" "We have a brand new Architect approved package that's just come in!" (`|MakeArray` "[Next]" :!type "Text")))
                          (switch `/Game/Blueprints/Enum_DialogueState` _state_63
                            (:`NewEnumerator0`
                              (goto _label_9))))))))))
            (:`3`
              (bind (_state_64 _optionindex_13) (`self.AddDialogue` "Travel Agent" "...Was there something else?" (`|MakeArray` "Nevermind, sorry" "Tell me more about what you were going to say" :!type "Text")))
              (switch `/Game/Blueprints/Enum_DialogueState` _state_64
                (:`NewEnumerator0`
                  (switch `int` _optionindex_13
                    (:`0`
                      (`self.ClearDialogueProgress`)
                      (`self.CloseConversation`))
                    (:`1`
                      (bind _state_65 (`self.AddDialogue` "Travel Agent" "Like I said, Sir, It's probably a bad idea..." (`|MakeArray` "It's okay, you can trust me" "Please, maybe I can help in some way..." :!type "Text")))
                      (switch `/Game/Blueprints/Enum_DialogueState` _state_65
                        (:`NewEnumerator0`
                          (goto _label_8))))))))))
        (:`2`
          (switch `int` (`self.DialogueTreeIndex`)
            (:`0`
              (bind _state_66 (`self.AddDialogue` "Travel Agent" "Plesantries, Sir! Can I interest you in a package holiday? " (`|MakeArray` "Has anyone...spoken with you?" "Are you feeling alright?" :!type "Text") :!label _label_11))
              (switch `/Game/Blueprints/Enum_DialogueState` _state_66
                (:`NewEnumerator0`
                  (bind _state_67 (`self.AddDialogue` "Travel Agent" "All the wonders of the world, right here within our borders!  " (`|MakeArray` "[Next]" :!type "Text")))
                  (switch `/Game/Blueprints/Enum_DialogueState` _state_67
                    (:`NewEnumerator0`
                      (bind _state_68 (`self.AddDialogue` "Travel Agent" "Golden fields, crystal rivers- the Ministry of Tourism calls it the Nation Eternal. Has a nice ring to it, don’t you think?" (`|MakeArray` "Are you listening to yourself?" "You seem...especially enthusiastic" :!type "Text")))
                      (switch `/Game/Blueprints/Enum_DialogueState` _state_68
                        (:`NewEnumerator0`
                          (bind _state_69 (`self.AddDialogue` "Travel Agent" "Well, you know what they say - there’s no place like home! Now... what can I book for you?" (`|MakeArray` "I’ll need to get going " "What have I done..." :!type "Text")))
                          (switch `/Game/Blueprints/Enum_DialogueState` _state_69
                            (:`NewEnumerator0`
                              (`self.SetDialogueTreeIndex` 4)
                              (`self.ClearDialogueProgress`)
                              (`self.CloseConversation`))))))))))
            (:`1`
              (goto _label_11))
            (:`2`
              (goto _label_11))
            (:`3`
              (goto _label_11))
            (:`4`
              (bind (_state_70 _optionindex_14) (`self.AddDialogue` "Travel Agent" "Plesantries, Sir! Can I interest you in a package holiday? " (`|MakeArray` "..." "[Close]" :!type "Text")))
              (switch `/Game/Blueprints/Enum_DialogueState` _state_70
                (:`NewEnumerator0`
                  (switch `int` _optionindex_14
                    (:`0`
                      (bind (_state_71 _optionindex_15) (`self.AddDialogue` "Travel Agent" "All the wonders of the world, right here within our borders!  " (`|MakeArray` "Please say something else" "[Close]" :!type "Text")))
                      (switch `/Game/Blueprints/Enum_DialogueState` _state_71
                        (:`NewEnumerator0`
                          (switch `int` _optionindex_15
                            (:`0`
                              (bind (_state_72 _optionindex_16) (`self.AddDialogue` "Travel Agent" "Golden fields, crystal rivers- the Ministry of Tourism calls it the Nation Eternal. Has a nice ring to it, don’t you think?" (`|MakeArray` "Please" "[Close]" :!type "Text")))
                              (switch `/Game/Blueprints/Enum_DialogueState` _state_72
                                (:`NewEnumerator0`
                                  (switch `int` _optionindex_16
                                    (:`0`
                                      (bind _state_73 (`self.AddDialogue` "Travel Agent" "Well, you know what they say - there’s no place like home! Now... what can I book for you?" (`|MakeArray` "Goodbye.. " "[Close]" :!type "Text")))
                                      (switch `/Game/Blueprints/Enum_DialogueState` _state_73
                                        (:`NewEnumerator0`
                                          (`self.ClearDialogueProgress`)
                                          (`self.CloseConversation`))))
                                    (:`1`
                                      (`self.ClearDialogueProgress`)
                                      (`self.CloseConversation`))))))
                            (:`1`
                              (`self.ClearDialogueProgress`)
                              (`self.CloseConversation`))))))
                    (:`1`
                      (`self.ClearDialogueProgress`)
                      (`self.CloseConversation`))))))))))))