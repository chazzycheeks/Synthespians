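; Branching dialogue for the Chairwoman NPC, a People's Committee loyalist who talks up the Architect's regime, its job program and a displayed Heretic.
; When the player is ready to phone, only a prompt to report in plays.
; Otherwise DialogueTreeIndex selects the first meeting, repeat greeting or a silent brush-off after the player voices sympathy.
; Chained AddDialogue calls branch on OptionIndex and share converging lines; endings clear progress and close the conversation.
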(fn `Dialogue`
  (`parent.Dialogue`)
  (bind _readytophone (`self.GetIsReadyToPhoneBool`))
  (if _readytophone
    (bind _state (`self.AddDialogue` "You" "I should report in at the phone." (`|MakeArray` "[Close]" :!type "Text")))
    (switch `/Game/Blueprints/Enum_DialogueState` _state
      (:`NewEnumerator0`
        (`self.ClearDialogueProgress`)
        (`self.CloseConversation`)))
    (else
      (switch `int` (`self.DialogueTreeIndex`)
        (:`0`
          (bind (_state_2 _optionindex) (`self.AddDialogue` "Chairwoman" "Pleasantries Sir!" (`|MakeArray` "Hello" "Pleasantries" :!type "Text")))
          (switch `/Game/Blueprints/Enum_DialogueState` _state_2
            (:`NewEnumerator0`
              (switch `int` _optionindex
                (:`0`
                  (bind (_state_3 _optionindex_2) (`self.AddDialogue` "Chairwoman" "I think the word you are looking for is 'Pleasantries', dear." (`|MakeArray` "Sounds similar enough" "Haven't they got the same meaning?" "Oh sorry-Pleasantries" :!type "Text")))
                  (switch `/Game/Blueprints/Enum_DialogueState` _state_3
                    (:`NewEnumerator0`
                      (switch `int` _optionindex_2
                        (:`0`
                          (bind _state_4 (`self.AddDialogue` "Chairwoman" "Perhaps.. to someone like you. Around here, we prefer the formality." (`|MakeArray` "[Next]" :!type "Text") :!label _label))
                          (switch `/Game/Blueprints/Enum_DialogueState` _state_4
                            (:`NewEnumerator0`
                              _)))
                        (:`1`
                          (goto _label))
                        (:`2`
                          (bind _state_5 (`self.AddDialogue` "Chairwoman" "That's better." (`|MakeArray` "[Next]" :!type "Text")))
                          (switch `/Game/Blueprints/Enum_DialogueState` _state_5
                            (:`NewEnumerator0`
                              _)))))))
                (:`1`
                  _))
              (bind _state_6 (`self.AddDialogue` "Chairwoman" " I can see from your attire that you aren’t from around here… What brings you to this district?" (`|MakeArray` "[Next]" :!type "Text")))
              (switch `/Game/Blueprints/Enum_DialogueState` _state_6
                (:`NewEnumerator0`
                  (bind (_state_7 _optionindex_3) (`self.AddDialogue` "Chairwoman" " It has been some time since we had a new face around here.. Always a pleasure." (`|MakeArray` "I'm just passing through" "I'm looking for work" "So you know everyone here?" :!type "Text")))
                  (switch `/Game/Blueprints/Enum_DialogueState` _state_7
                    (:`NewEnumerator0`
                      (switch `int` _optionindex_3
                        (:`0`
                          (bind _state_8 (`self.AddDialogue` "Chairwoman" " …A tourist? How novel. " (`|MakeArray` "[Next]" :!type "Text")))
                          (switch `/Game/Blueprints/Enum_DialogueState` _state_8
                            (:`NewEnumerator0`
                              (bind (_state_9 _optionindex_4) (`self.AddDialogue` "Chairwoman" "Well, pardon my surprise. As Chair of the P.C I am usually breifed on outside arrivals. " (`|MakeArray` "Do you know everything that goes on?" "Briefed by who?" "P.C?" :!type "Text")))
                              (switch `/Game/Blueprints/Enum_DialogueState` _state_9
                                (:`NewEnumerator0`
                                  (switch `int` _optionindex_4
                                    (:`0`
                                      (bind (_state_10 _optionindex_5) (`self.AddDialogue` "Chairwoman" "Some call it oversight - I prefer stewardship. Every name, every record, every movement passes through me eventually.. " (`|MakeArray` "Sounds a bit invasive" "Seems important" :!type "Text") :!label _label_2))
                                      (switch `/Game/Blueprints/Enum_DialogueState` _state_10
                                        (:`NewEnumerator0`
                                          (switch `int` _optionindex_5
                                            (:`0`
                                              (bind _state_11 (`self.AddDialogue` "Chairwoman" "Only to those who have something to hide." (`|MakeArray` "Such as.." "Like this person here?" :!type "Text")))
                                              (switch `/Game/Blueprints/Enum_DialogueState` _state_11
                                                (:`NewEnumerator0`
                                                  (bind _state_12 (`self.AddDialogue` "Chairwoman" "Our most recent Heretic." (`|MakeArray` "[Next]" :!type "Text") :!label _label_3))
                                                  (switch `/Game/Blueprints/Enum_DialogueState` _state_12
                                                    (:`NewEnumerator0`
                                                      _)))))
                                            (:`1`
                                              (bind (_state_13 _optionindex_6) (`self.AddDialogue` "Chairwoman" "That it most certainly is, dear! Helps avoid any further heretic activity. " (`|MakeArray` "Heretic activity?" "Has there been a lot of that as of late?" :!type "Text")))
                                              (switch `/Game/Blueprints/Enum_DialogueState` _state_13
                                                (:`NewEnumerator0`
                                                  (switch `int` _optionindex_6
                                                    (:`0`
                                                      (goto _label_3))
                                                    (:`1`
                                                      (bind _state_14 (`self.AddDialogue` "Chairwoman" "Goodness no, of course not! Only ever a couple foolish outliers. Such as our most recent case next to me." (`|MakeArray` "[Next]" :!type "Text")))
                                                      (switch `/Game/Blueprints/Enum_DialogueState` _state_14
                                                        (:`NewEnumerator0`
                                                          _))))))))
                                          (bind _state_15 (`self.AddDialogue` "Chairwoman" "Loathesome fellow. The state is quite right to dissuade others from his selfish path. " (`|MakeArray` "[Next]" :!type "Text")))
                                          (switch `/Game/Blueprints/Enum_DialogueState` _state_15
                                            (:`NewEnumerator0`
                                              (bind _state_16 (`self.AddDialogue` "Chairwoman" "The Architect believes in transparency, you see. A display of dishonesty keeps the rest of us steady." (`|MakeArray` "[Next]" :!type "Text")))
                                              (switch `/Game/Blueprints/Enum_DialogueState` _state_16
                                                (:`NewEnumerator0`
                                                  (bind (_state_17 _optionindex_7) (`self.AddDialogue` "Chairwoman" "It's already decreased Heretic activity by 90 percent! How fortunate we are to be rid of such a poison." (`|MakeArray` "What's his name?" "What did he do?" :!type "Text")))
                                                  (switch `/Game/Blueprints/Enum_DialogueState` _state_17
                                                    (:`NewEnumerator0`
                                                      (switch `int` _optionindex_7
                                                        (:`0`
                                                          (bind _state_18 (`self.AddDialogue` "Chairwoman" "Curiosity is a dangerous virtue, dear. He is a Heretic after all." (`|MakeArray` "[Next]" :!type "Text")))
                                                          (switch `/Game/Blueprints/Enum_DialogueState` _state_18
                                                            (:`NewEnumerator0`
                                                              _)))
                                                        (:`1`
                                                          (bind _state_19 (`self.AddDialogue` "Chairwoman" "Curiosity is a dangerous virtue, dear. I wouldn't wish to catch you being sympathetic now… " (`|MakeArray` "[Next]" :!type "Text")))
                                                          (switch `/Game/Blueprints/Enum_DialogueState` _state_19
                                                            (:`NewEnumerator0`
                                                              _))))
                                                      (bind _state_20 (`self.AddDialogue` "Chairwoman" "Have a pleasant day stranger.  " (`|MakeArray` "[Close]" :!type "Text")))
                                                      (switch `/Game/Blueprints/Enum_DialogueState` _state_20
                                                        (:`NewEnumerator0`
                                                          (`self.SetDialogueTreeIndex` 1)
                                                          (`self.ClearDialogueProgress`)
                                                          (`self.CloseConversation`))))))))))))
                                    (:`1`
                                      (bind _state_21 (`self.AddDialogue` "Chairwoman" "Aren't you the curious type. That's a dangerous type to be." (`|MakeArray` "[Next]" :!type "Text")))
                                      (switch `/Game/Blueprints/Enum_DialogueState` _state_21
                                        (:`NewEnumerator0`
                                          (bind _state_22 (`self.AddDialogue` "Chairwoman" "Have a pleasant day now, stranger." (`|MakeArray` "[Close]" :!type "Text")))
                                          (switch `/Game/Blueprints/Enum_DialogueState` _state_22
                                            (:`NewEnumerator0`
                                              (`self.SetDialogueTreeIndex` 1)
                                              (`self.ClearDialogueProgress`)
                                              (`self.CloseConversation`))))))
                                    (:`2`
                                      (bind _state_23 (`self.AddDialogue` "Chairwoman" "The People's Comittee. A State funded body of like minded patriots, such as myself, reporting directly to the Inner Sector." (`|MakeArray` "You must know all the goings on then?" "Sounds... important" :!type "Text")))
                                      (switch `/Game/Blueprints/Enum_DialogueState` _state_23
                                        (:`NewEnumerator0`
                                          (goto _label_2))))))))))
                        (:`1`
                          (bind _state_24 (`self.AddDialogue` "Chairwoman" " Of course you are! Wonderful." (`|MakeArray` "[Next]" :!type "Text")))
                          (switch `/Game/Blueprints/Enum_DialogueState` _state_24
                            (:`NewEnumerator0`
                              (bind _state_25 (`self.AddDialogue` "Chairwoman" "Well, you have come to the right place! " (`|MakeArray` "[Next]" :!type "Text")))
                              (switch `/Game/Blueprints/Enum_DialogueState` _state_25
                                (:`NewEnumerator0`
                                  (bind _state_26 (`self.AddDialogue` "Chairwoman" "Starting tomorrow, we have the new Employment Boost Program." (`|MakeArray` "[Next]" :!type "Text")))
                                  (switch `/Game/Blueprints/Enum_DialogueState` _state_26
                                    (:`NewEnumerator0`
                                      (bind (_state_27 _optionindex_8) (`self.AddDialogue` "Chairwoman" "The Architect himself approved it. Isn’t that something? Always thinking of his people." (`|MakeArray` "A generous man, indeed" "His people… like this person here? " "What's the program?" :!type "Text")))
                                      (switch `/Game/Blueprints/Enum_DialogueState` _state_27
                                        (:`NewEnumerator0`
                                          (switch `int` _optionindex_8
                                            (:`0`
                                              (bind _state_28 (`self.AddDialogue` "Chairwoman" "  As he always says, generosity is the foundation of freedom." (`|MakeArray` "[Next]" :!type "Text")))
                                              (switch `/Game/Blueprints/Enum_DialogueState` _state_28
                                                (:`NewEnumerator0`
                                                  (bind (_state_29 _optionindex_9) (`self.AddDialogue` "Chairwoman" " And look how we’re living now. Clean air. Quiet streets... These are truly blessed times. " (`|MakeArray` "We are truly lucky" "Yeah.." :!type "Text")))
                                                  (switch `/Game/Blueprints/Enum_DialogueState` _state_29
                                                    (:`NewEnumerator0`
                                                      (switch `int` _optionindex_9
                                                        (:`0`
                                                          (bind _state_30 (`self.AddDialogue` "Chairwoman" "That we are! You have a blessed day now." (`|MakeArray` "[Close]" :!type "Text")))
                                                          (switch `/Game/Blueprints/Enum_DialogueState` _state_30
                                                            (:`NewEnumerator0`
                                                              (`self.SetDialogueTreeIndex` 1)
                                                              (`self.ClearDialogueProgress`)
                                                              (`self.CloseConversation`))))
                                                        (:`1`
                                                          (bind _state_31 (`self.AddDialogue` "Chairwoman" "You have a blessed day now." (`|MakeArray` "[Close]" :!type "Text") :!label _label_4))
                                                          (switch `/Game/Blueprints/Enum_DialogueState` _state_31
                                                            (:`NewEnumerator0`
                                                              (`self.SetDialogueTreeIndex` 1)
                                                              (`self.ClearDialogueProgress`)
                                                              (`self.CloseConversation`))))))))))
                                            (:`1`
                                              (goto _label_3))
                                            (:`2`
                                              (bind _state_32 (`self.AddDialogue` "Chairwoman" "Just a few minor enahncements to our existing formula, to ensure everyone’s doing their part." (`|MakeArray` "[Next]" :!type "Text")))
                                              (switch `/Game/Blueprints/Enum_DialogueState` _state_32
                                                (:`NewEnumerator0`
                                                  (bind (_state_33 _optionindex_10) (`self.AddDialogue` "Chairwoman" "Efficiency audits, reallocation of labor. Waste is such an ugly thing, don’t you agree?" (`|MakeArray` "Of course" "Depends what you mean by 'waste'" :!type "Text")))
                                                  (switch `/Game/Blueprints/Enum_DialogueState` _state_33
                                                    (:`NewEnumerator0`
                                                      (switch `int` _optionindex_10
                                                        (:`0`
                                                          (bind _state_34 (`self.AddDialogue` "Chairwoman" "I am most pleased you agree!" (`|MakeArray` "[Next]" :!type "Text")))
                                                          (switch `/Game/Blueprints/Enum_DialogueState` _state_34
                                                            (:`NewEnumerator0`
                                                              _)))
                                                        (:`1`
                                                          (bind _state_35 (`self.AddDialogue` "Chairwoman" "Only those that do not pull their weight. After all the Architect has provided for them, it is the least they can do in return. " (`|MakeArray` "[Next]" :!type "Text")))
                                                          (switch `/Game/Blueprints/Enum_DialogueState` _state_35
                                                            (:`NewEnumerator0`
                                                              _))))
                                                      (bind _state_36 (`self.AddDialogue` "Chairwoman" "Shall I begin the process of getting you signed up?" (`|MakeArray` "Not right now" "Maybe later" :!type "Text")))
                                                      (switch `/Game/Blueprints/Enum_DialogueState` _state_36
                                                        (:`NewEnumerator0`
                                                          (bind _state_37 (`self.AddDialogue` "Chairwoman" "Well act fast! The first 100 people to sign up are granted FIVE bonus ration vouchers during their first month! " (`|MakeArray` "[Next]" :!type "Text")))
                                                          (switch `/Game/Blueprints/Enum_DialogueState` _state_37
                                                            (:`NewEnumerator0`
                                                              (goto _label_4))))))))))))))))))))
                        (:`2`
                          (goto _label_2))))))))))
        (:`1`
          (bind (_state_38 _optionindex_11) (`self.AddDialogue` "Chairwoman" "Pleasantries! Is there something else I can help you with?" (`|MakeArray` "No that's alright" "Can you tell me more about this Heretic?" :!type "Text")))
          (switch `/Game/Blueprints/Enum_DialogueState` _state_38
            (:`NewEnumerator0`
              (switch `int` _optionindex_11
                (:`0`
                  (bind _state_39 (`self.AddDialogue` "Chairwoman" "Have a pleasant day.  " (`|MakeArray` "[Close]" :!type "Text")))
                  (switch `/Game/Blueprints/Enum_DialogueState` _state_39
                    (:`NewEnumerator0`
                      (`self.ClearDialogueProgress`)
                      (`self.CloseConversation`))))
                (:`1`
                  (bind _state_40 (`self.AddDialogue` "Chairwoman" "Well deary, he is a foul-mouthed dirty criminal. " (`|MakeArray` "[Next]" :!type "Text")))
                  (switch `/Game/Blueprints/Enum_DialogueState` _state_40
                    (:`NewEnumerator0`
                      (bind _state_41 (`self.AddDialogue` "Chairwoman" "Speaking against the Architects utopia, the fool. " (`|MakeArray` "[Next]" :!type "Text")))
                      (switch `/Game/Blueprints/Enum_DialogueState` _state_41
                        (:`NewEnumerator0`
                          (bind (_state_42 _optionindex_12) (`self.AddDialogue` "Chairwoman" "Now he'll never speak again, thank the Architect. " (`|MakeArray` "Thank him, indeed" "...That seems quite cruel" :!type "Text")))
                          (switch `/Game/Blueprints/Enum_DialogueState` _state_42
                            (:`NewEnumerator0`
                              (switch `int` _optionindex_12
                                (:`0`
                                  (bind _state_43 (`self.AddDialogue` "Chairwoman" "And our country is a better place for it! " (`|MakeArray` "[Next]" :!type "Text")))
                                  (switch `/Game/Blueprints/Enum_DialogueState` _state_43
                                    (:`NewEnumerator0`
                                      (bind _state_44 (`self.AddDialogue` "Chairwoman" "You have a pleasant day now." (`|MakeArray` "[Close]" :!type "Text")))
                                      (switch `/Game/Blueprints/Enum_DialogueState` _state_44
                                        (:`NewEnumerator0`
                                          (`self.ClearDialogueProgress`)
                                          (`self.CloseConversation`))))))
                                (:`1`
                                  (bind _state_45 (`self.AddDialogue` "Chairwoman" "..." (`|MakeArray` "[Next]" :!type "Text")))
                                  (switch `/Game/Blueprints/Enum_DialogueState` _state_45
                                    (:`NewEnumerator0`
                                      (bind _state_46 (`self.AddDialogue` "Chairwoman" "I'm sorry dear, I must be hearing things." (`|MakeArray` "[Next]" :!type "Text")))
                                      (switch `/Game/Blueprints/Enum_DialogueState` _state_46
                                        (:`NewEnumerator0`
                                          (bind _state_47 (`self.AddDialogue` "Chairwoman" "I have to go now.." (`|MakeArray` "[Next]" :!type "Text")))
                                          (switch `/Game/Blueprints/Enum_DialogueState` _state_47
                                            (:`NewEnumerator0`
                                              (bind _state_48 (`self.AddDialogue` "Chairwoman" "Goodbye." (`|MakeArray` "[Close]" :!type "Text")))
                                              (switch `/Game/Blueprints/Enum_DialogueState` _state_48
                                                (:`NewEnumerator0`
                                                  (`self.SetDialogueTreeIndex` 2)
                                                  (`self.ClearDialogueProgress`)
                                                  (`self.CloseConversation`))))))))))))))))))))))
        (:`2`
          (bind _state_49 (`self.AddDialogue` "Chairwoman" ".." (`|MakeArray` "[Close]" :!type "Text")))
          (switch `/Game/Blueprints/Enum_DialogueState` _state_49
            (:`NewEnumerator0`
              (`self.ClearDialogueProgress`)
              (`self.CloseConversation`))))))))