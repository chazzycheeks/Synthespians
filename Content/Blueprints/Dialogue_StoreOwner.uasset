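; Dialogue script for the store owner NPC (speaker "Florist"), with placeholder-style test lines, overriding a parent Dialogue function.
; DialogueTreeIndex selects a branching first conversation or one of two follow-up trees that give a random hostile brush-off.
; Chained AddDialogue calls advance on Pass Through and branch on the chosen option.
; Certain endings change the tree index, clear dialogue progress or increment level progress; the last tree has nothing wired after its line.
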(fn `Dialogue`
  (`parent.Dialogue`)
  (switch `int` (`self.DialogueTreeIndex`)
    (:`0`
      (bind (_state _optionindex) (`self.AddDialogue` "Florist" "Hello this is a test" (`|MakeArray` "cool" "go away" :!type "Text")))
      (switch `/Game/Blueprints/Enum_DialogueState` _state
        (:`NewEnumerator0`
          (switch `int` _optionindex
            (:`0`
              (bind (_state_2 _optionindex_2) (`self.AddDialogue` "Florist" "Cool is right" (`|MakeArray` "cool again" "yeah" :!type "Text")))
              (switch `/Game/Blueprints/Enum_DialogueState` _state_2
                (:`NewEnumerator0`
                  (switch `int` _optionindex_2
                    (:`0`
                      (bind (_state_3 _optionindex_3) (`self.AddDialogue` "Florist" "yes ok i get it" (`|MakeArray` "sorry" "COOL" :!type "Text")))
                      (switch `/Game/Blueprints/Enum_DialogueState` _state_3
                        (:`NewEnumerator0`
                          (switch `int` _optionindex_3
                            (:`0`
                              (bind _state_4 (`self.AddDialogue` "Florist" "Thats ok" (`|MakeArray` "Continue" :!type "Text")))
                              (switch `/Game/Blueprints/Enum_DialogueState` _state_4
                                (:`NewEnumerator0`
                                  (bind _state_5 (`self.AddDialogue` "Florist" "Maybe chill next time" (`|MakeArray` "Close" :!type "Text")))
                                  (switch `/Game/Blueprints/Enum_DialogueState` _state_5
                                    (:`NewEnumerator0`
                                      (`self.IncrementLevelProgress`)
                                      (`self.SetDialogueTreeIndex` 2)
                                      (`self.ClearDialogueProgress`)
                                      (`self.CloseConversation`))))))
                            (:`1`
                              (bind _state_6 (`self.AddDialogue` "Florist" "Stay away from me" (`|MakeArray` "End" :!type "Text")))
                              (switch `/Game/Blueprints/Enum_DialogueState` _state_6
                                (:`NewEnumerator0`
                                  (`self.CloseConversation`))))))))
                    (:`1`
                      (`self.ClearDialogueProgress`)
                      (`self.CloseConversation`))))))
            (:`1`
              (bind _state_7 (`self.AddDialogue` "Florist" "Ok bitch" (`|MakeArray` "End" :!type "Text")))
              (switch `/Game/Blueprints/Enum_DialogueState` _state_7
                (:`NewEnumerator0`
                  (`self.SetDialogueTreeIndex` 1)
                  (`self.CloseConversation`))))))))
    (:`1`
      (bind _state_8 (`self.AddDialogue` "Florist" (select `int` (`KismetMathLibrary.RandomIntegerInRange` 0 1) :`0` "Fuck you" :`1` "go away" :!type "Text") (`|MakeArray` "End" :!type "Text")))
      (switch `/Game/Blueprints/Enum_DialogueState` _state_8
        (:`NewEnumerator0`
          (`self.ClearDialogueProgress`)
          (`self.CloseConversation`)
          (`self.IncrementLevelProgress`))))
    (:`2`
      (bind _state_9 (`self.AddDialogue` "Florist" (select `int` (`KismetMathLibrary.RandomIntegerInRange` 0 1) :`0` "Fuck you" :`1` "go away" :!type "Text") (`|MakeArray` "End" :!type "Text")))
      (switch `/Game/Blueprints/Enum_DialogueState` _state_9))))