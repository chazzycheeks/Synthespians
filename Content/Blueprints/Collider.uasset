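; Collider is a trigger actor that starts a dialogue when the first-person player character overlaps it.
; If its Available flag is set, it opens a conversation through DialoguePlayer, switches input to UI only, shows the mouse cursor and disables the character's movement.
; It also sets IsTheCollider on the character; nothing in this graph clears Available or restores movement and input.
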(event `self.ReceiveActorBeginOverlap`
  (params (OtherActor :type "Actor Object Reference"))
  (bind _asbp_first_person_character (cast `/Game/FirstPerson/Blueprints/BP_FirstPersonCharacter` OtherActor))
  (if (`self.Available`)
    (`/Game/Blueprints/AC_dialogue_base.OpenConversation` (`self.Dialogue_Player`))
    (`WidgetBlueprintLibrary.SetInputMode_UIOnlyEx` (`GameplayStatics.GetPlayerController` 0) null)
    (`CharacterMovementComponent.SetMovementMode` (`Character.CharacterMovement` _asbp_first_person_character) "MOVE_None" 0)
    (set `PlayerController.bShowMouseCursor` true (`GameplayStatics.GetPlayerController` 0))
    (set `/Game/FirstPerson/Blueprints/BP_FirstPersonCharacter.IsTheCollider` true _asbp_first_person_character)))

(fn `UserConstructionScript`)