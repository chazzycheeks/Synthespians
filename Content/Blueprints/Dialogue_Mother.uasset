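; Dialogue for the Mother NPC, a branching conversation about motherhood under the State and her daughter Lily.
; Dialogue calls its parent, gives a phone reminder when the ready-to-phone flag is set, otherwise branches on level progress and DialogueTreeIndex.
; Nested AddDialogue nodes route on chosen options, with some branches rejoining.
; Endings store the tree index for return visits, or advance level progress and set the phone flag.
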(fn `Dialogue`
  (`parent.Dialogue`)
  (bind _readytophone (`self.GetIsReadyToPhoneBool`))
  (if _readytophone
    (bind _state (`self.AddDialogue` "You" "I should report in at the phone." (`|MakeArray` "[Close]" :!type "Text")))
    (switch `/Game/Blueprints/Enum_DialogueState` _state
      (:`NewEnumerator0`
        (`self.ClearDialogueProgress`)
        (`self.CloseConversation`)))
    (else
      (bind _this_index (`self.GetLevelProgressIndex`))
      (switch `int` _this_index
        (:`0`
          (switch `int` (`self.DialogueTreeIndex`) :!label _label
            (:`0`
              (bind _state_2 (`self.AddDialogue` "Mother" "... Pleasantries. Can I..help you with something?" (`|MakeArray` "Thought I'd say hello" "Sorry, are you busy?" :!type "Text")))
              (switch `/Game/Blueprints/Enum_DialogueState` _state_2
                (:`NewEnumerator0`
                  (bind _state_3 (`self.AddDialogue` "Mother" "Sorry I'm actually on the school run but.." (`|MakeArray` "[Next]" :!type "Text")))
                  (switch `/Game/Blueprints/Enum_DialogueState` _state_3
                    (:`NewEnumerator0`
                      (bind _state_4 (`self.AddDialogue` "Mother" "I got distracted.." (`|MakeArray` "[Next]" :!type "Text")))
                      (switch `/Game/Blueprints/Enum_DialogueState` _state_4
                        (:`NewEnumerator0`
                          (bind _state_5 (`self.AddDialogue` "Mother" "I should go, but maybe we'll catch each other another time." (`|MakeArray` "[Close]" :!type "Text")))
                          (switch `/Game/Blueprints/Enum_DialogueState` _state_5
                            (:`NewEnumerator0`
                              (`self.SetDialogueTreeIndex` 1)
                              (`self.ClearDialogueProgress`)
                              (`self.CloseConversation`))))))))))
            (:`1`
              (bind _state_6 (`self.AddDialogue` "Mother" "I must go, sorry." (`|MakeArray` "[Close]" :!type "Text")))
              (switch `/Game/Blueprints/Enum_DialogueState` _state_6
                (:`NewEnumerator0`
                  (`self.ClearDialogueProgress`)
                  (`self.CloseConversation`))))))
        (:`1`
          (goto _label))
        (:`2`
          (switch `int` (`self.DialogueTreeIndex`)
            (:`0`
              (bind _state_7 (`self.AddDialogue` "Mother" "..." (`|MakeArray` "Hello?" "Pleasantries" :!type "Text")))
              (switch `/Game/Blueprints/Enum_DialogueState` _state_7
                (:`NewEnumerator0`
                  (bind (_state_8 _optionindex) (`self.AddDialogue` "Mother" " Oh- pleasantries. Apologies, my mind was elsewhere." (`|MakeArray` "Didn’t mean to catch you off guard" "My fault" "What were you thinking about?" :!type "Text")))
                  (switch `/Game/Blueprints/Enum_DialogueState` _state_8
                    (:`NewEnumerator0`
                      (switch `int` _optionindex
                        (:`0`
                          _)
                        (:`1`
                          _)
                        (:`2`
                          (bind _state_9 (`self.AddDialogue` "Mother" "Oh- nothing." (`|MakeArray` "[Next]" :!type "Text")))
                          (switch `/Game/Blueprints/Enum_DialogueState` _state_9
                            (:`NewEnumerator0`
                              _))))
                      (bind _state_10 (`self.AddDialogue` "Mother" "You must be new. Couldn’t have been here more than a few days." (`|MakeArray` "What makes you say that?" "How did you know?" :!type "Text")))
                      (switch `/Game/Blueprints/Enum_DialogueState` _state_10
                        (:`NewEnumerator0`
                          (bind (_state_11 _optionindex_2) (`self.AddDialogue` "Mother" "You see most keep to themselves these days. The Chairwoman doesn’t ‘appreciate’ loitering.  " (`|MakeArray` "Nor should she" "A shame..." "You been here long?" :!type "Text")))
                          (switch `/Game/Blueprints/Enum_DialogueState` _state_11
                            (:`NewEnumerator0`
                              (switch `int` _optionindex_2
                                (:`0`
                                  (bind _state_12 (`self.AddDialogue` "Mother" "Right…" (`|MakeArray` "[Next]" :!type "Text")))
                                  (switch `/Game/Blueprints/Enum_DialogueState` _state_12
                                    (:`NewEnumerator0`
                                      (bind _state_13 (`self.AddDialogue` "Mother" "Well, I’ll need to be getting home. Jobs to attend to. You have a pleasant day, Sir." (`|MakeArray` "[Close]" :!type "Text")))
                                      (switch `/Game/Blueprints/Enum_DialogueState` _state_13
                                        (:`NewEnumerator0`
                                          (`self.SetDialogueTreeIndex` 1)
                                          (`self.ClearDialogueProgress`)
                                          (`self.CloseConversation`))))))
                                (:`1`
                                  (bind _state_14 (`self.AddDialogue` "Mother" "It can certainly get lonely. Suppose it makes me all the more grateful for my Lily." (`|MakeArray` "Lily?" "Your daughter?" :!type "Text")))
                                  (switch `/Game/Blueprints/Enum_DialogueState` _state_14
                                    (:`NewEnumerator0`
                                      (bind _state_15 (`self.AddDialogue` "Mother" "Yes. Seven next month. You’ll hear her before you see her, she’s got that kind of laugh." (`|MakeArray` "You must be very proud" "She must like it here then?" :!type "Text") :!label _label_2))
                                      (switch `/Game/Blueprints/Enum_DialogueState` _state_15
                                        (:`NewEnumerator0`
                                          (switch `int` 0
                                            (:`0`
                                              (bind _state_16 (`self.AddDialogue` "Mother" "More than I could possibly say. She really is the brightest little soul. Excited, carefree...." (`|MakeArray` "[Next]" :!type "Text")))
                                              (switch `/Game/Blueprints/Enum_DialogueState` _state_16
                                                (:`NewEnumerator0`
                                                  (bind _state_17 (`self.AddDialogue` "Mother" "Suppose thats why its all so- terrifying.  " (`|MakeArray` "Terrifying?" "What do you mean?" :!type "Text")))
                                                  (switch `/Game/Blueprints/Enum_DialogueState` _state_17
                                                    (:`NewEnumerator0`
                                                      (bind _state_18 (`self.AddDialogue` "Mother" "Just… the state of things. The opportunities she’ll have here." (`|MakeArray` "Are they not good?" "There's plenty of time!" :!type "Text")))
                                                      (switch `/Game/Blueprints/Enum_DialogueState` _state_18
                                                        (:`NewEnumerator0`
                                                          (bind _state_19 (`self.AddDialogue` "Mother" "You really are new..." (`|MakeArray` "Did you always want to be a mother?" "Didn't you want to have kids?" :!type "Text")))
                                                          (switch `/Game/Blueprints/Enum_DialogueState` _state_19
                                                            (:`NewEnumerator0`
                                                              (bind _state_20 (`self.AddDialogue` "Mother" "..." (`|MakeArray` "[Next]" :!type "Text") :!label _label_3))
                                                              (switch `/Game/Blueprints/Enum_DialogueState` _state_20
                                                                (:`NewEnumerator0`
                                                                  (bind _state_21 (`self.AddDialogue` "Mother" "Sir... some conversations aren’t meant for the street. You never know who's listening, or..." (`|MakeArray` "[Next]" :!type "Text")))
                                                                  (switch `/Game/Blueprints/Enum_DialogueState` _state_21
                                                                    (:`NewEnumerator0`
                                                                      (bind (_state_22 _optionindex_3) (`self.AddDialogue` "Mother" "...Who exactly you’re talking to." (`|MakeArray` "I’m only asking because I care" "I’ve got my own issues with the State, trust me" "You're right, maybe we should stop" :!type "Text")))
                                                                      (switch `/Game/Blueprints/Enum_DialogueState` _state_22
                                                                        (:`NewEnumerator0`
                                                                          (switch `int` _optionindex_3
                                                                            (:`0`
                                                                              (bind _state_23 (`self.AddDialogue` "Mother" "Ok...You’re asking me about 'choice'… but that word’s lost all meaning." (`|MakeArray` "[Next]" :!type "Text") :!label _label_4))
                                                                              (switch `/Game/Blueprints/Enum_DialogueState` _state_23
                                                                                (:`NewEnumerator0`
                                                                                  (bind _state_24 (`self.AddDialogue` "Mother" "Motherhood is an expectation, the same way we expect rainfall or mandatory labour." (`|MakeArray` "[Next]" :!type "Text")))
                                                                                  (switch `/Game/Blueprints/Enum_DialogueState` _state_24
                                                                                    (:`NewEnumerator0`
                                                                                      (bind _state_25 (`self.AddDialogue` "Mother" "When I first discovered I was pregnant... " (`|MakeArray` "[Next]" :!type "Text")))
                                                                                      (switch `/Game/Blueprints/Enum_DialogueState` _state_25
                                                                                        (:`NewEnumerator0`
                                                                                          (bind _state_26 (`self.AddDialogue` "Mother" "...I tried everything to get rid of her.  " (`|MakeArray` "[Next]" :!type "Text")))
                                                                                          (switch `/Game/Blueprints/Enum_DialogueState` _state_26
                                                                                            (:`NewEnumerator0`
                                                                                              (bind (_state_27 _optionindex_4) (`self.AddDialogue` "Mother" "The old tricks... Boiling hot bath, too little to eat. But Lily came anyway. She's always been stubborn." (`|MakeArray` "That's- I'm so sorry.." "You have to have a baby?" :!type "Text")))
                                                                                              (switch `/Game/Blueprints/Enum_DialogueState` _state_27
                                                                                                (:`NewEnumerator0`
                                                                                                  (switch `int` _optionindex_4
                                                                                                    (:`0`
                                                                                                      (bind _state_28 (`self.AddDialogue` "Mother" "And yet I smile." (`|MakeArray` "[Next]" :!type "Text")))
                                                                                                      (switch `/Game/Blueprints/Enum_DialogueState` _state_28
                                                                                                        (:`NewEnumerator0`
                                                                                                          (bind _state_29 (`self.AddDialogue` "Mother" "And I send her off in her little uniform, and I tell her she’s lucky. " (`|MakeArray` "[Next]" :!type "Text")))
                                                                                                          (switch `/Game/Blueprints/Enum_DialogueState` _state_29
                                                                                                            (:`NewEnumerator0`
                                                                                                              (bind _state_30 (`self.AddDialogue` "Mother" "Because that’s what they want me to say. She thinks her mother can protect her..." (`|MakeArray` "[Next]" :!type "Text")))
                                                                                                              (switch `/Game/Blueprints/Enum_DialogueState` _state_30
                                                                                                                (:`NewEnumerator0`
                                                                                                                  (bind _state_31 (`self.AddDialogue` "Mother" "How could I tell her whats waiting? That she'll be starting mothering classes next year? I can't bear the thought." (`|MakeArray` "[Next]" :!type "Text")))
                                                                                                                  (switch `/Game/Blueprints/Enum_DialogueState` _state_31
                                                                                                                    (:`NewEnumerator0`
                                                                                                                      (bind _state_32 (`self.AddDialogue` "Mother" "So what can I do? Nothing. One step out of line and I'll have my mouth sewn shut just like this poor soul here, and never get to talk to her again." (`|MakeArray` "Have you thought about running?" "I hear there are maps, underground paths. " :!type "Text")))
                                                                                                                      (switch `/Game/Blueprints/Enum_DialogueState` _state_32
                                                                                                                        (:`NewEnumerator0`
                                                                                                                          _)))))))))))
                                                                                                    (:`1`
                                                                                                      (bind _state_33 (`self.AddDialogue` "Mother" "They call it ‘giving back’. We get notices printed on the backs of our ration cards, little reminders to keep the Nation growing. " (`|MakeArray` "[Next]" :!type "Text")))
                                                                                                      (switch `/Game/Blueprints/Enum_DialogueState` _state_33
                                                                                                        (:`NewEnumerator0`
                                                                                                          (bind _state_34 (`self.AddDialogue` "Mother" " Do you know the average woman here produces six children? Six. I can count myself lucky not be one of those." (`|MakeArray` "[Next]" :!type "Text")))
                                                                                                          (switch `/Game/Blueprints/Enum_DialogueState` _state_34
                                                                                                            (:`NewEnumerator0`
                                                                                                              (bind _state_35 (`self.AddDialogue` "Mother" "Of course, Government workers are exempt, but women rarely get chosen for that. " (`|MakeArray` "Have you thought about running?" "I hear there are maps, underground paths. " :!type "Text")))
                                                                                                              (switch `/Game/Blueprints/Enum_DialogueState` _state_35
                                                                                                                (:`NewEnumerator0`
                                                                                                                  _))))))))
                                                                                                  (bind _state_36 (`self.AddDialogue` "Mother" "And where would we go? The State keeps everything now- passports, food, medicine." (`|MakeArray` "[Next]" :!type "Text")))
                                                                                                  (switch `/Game/Blueprints/Enum_DialogueState` _state_36
                                                                                                    (:`NewEnumerator0`
                                                                                                      (bind _state_37 (`self.AddDialogue` "Mother" "Lily’s a diabetic... she’d die before we crossed the first border.  " (`|MakeArray` "That's so unbearable..." "How does anyone put up with this?" :!type "Text")))
                                                                                                      (switch `/Game/Blueprints/Enum_DialogueState` _state_37
                                                                                                        (:`NewEnumerator0`
                                                                                                          (bind _state_38 (`self.AddDialogue` "Mother" " You’d be surprised what people can bear. " (`|MakeArray` "[Next]" :!type "Text")))
                                                                                                          (switch `/Game/Blueprints/Enum_DialogueState` _state_38
                                                                                                            (:`NewEnumerator0`
                                                                                                              (bind _state_39 (`self.AddDialogue` "Mother" "You know… when I was a girl, they made us carry sacks of grain twice our weight.  " (`|MakeArray` "[Next]" :!type "Text")))
                                                                                                              (switch `/Game/Blueprints/Enum_DialogueState` _state_39
                                                                                                                (:`NewEnumerator0`
                                                                                                                  (bind _state_40 (`self.AddDialogue` "Mother" "We laughed about it, told it was some old tradition. Now I see it was practice." (`|MakeArray` "Practice?" "For what?" :!type "Text")))
                                                                                                                  (switch `/Game/Blueprints/Enum_DialogueState` _state_40
                                                                                                                    (:`NewEnumerator0`
                                                                                                                      (bind _state_41 (`self.AddDialogue` "Mother" "To carry the future of the State until our backs give out" (`|MakeArray` "[Next]" :!type "Text")))
                                                                                                                      (switch `/Game/Blueprints/Enum_DialogueState` _state_41
                                                                                                                        (:`NewEnumerator0`
                                                                                                                          (bind _state_42 (`self.AddDialogue` "Mother" "After that it's 'retirement' until the rest of our bodies follow suit. Then, finally, its back to the fields...to the grave. " (`|MakeArray` "[Next]" :!type "Text")))
                                                                                                                          (switch `/Game/Blueprints/Enum_DialogueState` _state_42
                                                                                                                            (:`NewEnumerator0`
                                                                                                                              (bind _state_43 (`self.AddDialogue` "Mother" "That’s what’s waiting for us... for my Lily." (`|MakeArray` "[Next]" :!type "Text")))
                                                                                                                              (switch `/Game/Blueprints/Enum_DialogueState` _state_43
                                                                                                                                (:`NewEnumerator0`
                                                                                                                                  (bind _state_44 (`self.AddDialogue` "Mother" "Now please excuse me..." (`|MakeArray` "[Next]" :!type "Text")))
                                                                                                                                  (switch `/Game/Blueprints/Enum_DialogueState` _state_44
                                                                                                                                    (:`NewEnumerator0`
                                                                                                                                      (bind _state_45 (`self.AddDialogue` "Mother" "I want to go see her... " (`|MakeArray` "[Close]" :!type "Text")))
                                                                                                                                      (switch `/Game/Blueprints/Enum_DialogueState` _state_45
                                                                                                                                        (:`NewEnumerator0`
                                                                                                                                          (`self.SetLevelProgressIndex` 3)
                                                                                                                                          (`self.SetIsReadyToPhoneBool` true)
                                                                                                                                          (`self.ClearDialogueProgress`)
                                                                                                                                          (`self.CloseConversation`))))))))))))))))))))))))))))))))
                                                                            (:`1`
                                                                              (goto _label_4))
                                                                            (:`2`
                                                                              (bind _state_46 (`self.AddDialogue` "Mother" "Right..." (`|MakeArray` "[Next]" :!type "Text")))
                                                                              (switch `/Game/Blueprints/Enum_DialogueState` _state_46
                                                                                (:`NewEnumerator0`
                                                                                  (bind _state_47 (`self.AddDialogue` "Mother" " I-I’ll need to be getting home. You have a pleasant day, Sir..." (`|MakeArray` "[Close]" :!type "Text")))
                                                                                  (switch `/Game/Blueprints/Enum_DialogueState` _state_47
                                                                                    (:`NewEnumerator0`
                                                                                      (`self.SetDialogueTreeIndex` 3)
                                                                                      (`self.ClearDialogueProgress`)
                                                                                      (`self.CloseConversation`))))))))))))))))))))))
                                            (:`1`
                                              (bind (_state_48 _optionindex_5) (`self.AddDialogue` "Mother" "For now... Yes." (`|MakeArray` "Before the State gets involved?" "Things seem to change fast around here" :!type "Text")))
                                              (switch `/Game/Blueprints/Enum_DialogueState` _state_48
                                                (:`NewEnumerator0`
                                                  (switch `int` _optionindex_5
                                                    (:`0`
                                                      (bind _state_49 (`self.AddDialogue` "Mother" " I-I’ll need to be getting home. Jobs to attend to. You have a pleasant day sir, look after yourself. " (`|MakeArray` "[Close]" :!type "Text")))
                                                      (switch `/Game/Blueprints/Enum_DialogueState` _state_49
                                                        (:`NewEnumerator0`
                                                          (`self.SetDialogueTreeIndex` 2)
                                                          (`self.ClearDialogueProgress`)
                                                          (`self.CloseConversation`))))
                                                    (:`1`
                                                      (bind _state_50 (`self.AddDialogue` "Mother" "That’s one way of putting it..." (`|MakeArray` "Did you always want to be a mother?" "Didn't you want to have kids?" :!type "Text")))
                                                      (switch `/Game/Blueprints/Enum_DialogueState` _state_50
                                                        (:`NewEnumerator0`
                                                          (goto _label_3))))))))))))))
                                (:`2`
                                  (bind _state_51 (`self.AddDialogue` "Mother" "A while. Feels longer, some days. My husband works at the co-op. I keep the house, look after Lily." (`|MakeArray` "Lily?" "Your daughter?" :!type "Text")))
                                  (switch `/Game/Blueprints/Enum_DialogueState` _state_51
                                    (:`NewEnumerator0`
                                      (goto _label_2))))))))))))))
            (:`1`
              (bind (_state_52 _optionindex_6) (`self.AddDialogue` "Mother" "...Pleasantries, was there something else?" (`|MakeArray` "It was a bad joke, my apologies" "Nothing, nevermind" :!type "Text")))
              (switch `/Game/Blueprints/Enum_DialogueState` _state_52
                (:`NewEnumerator0`
                  (switch `int` _optionindex_6
                    (:`0`
                      (bind _state_53 (`self.AddDialogue` "Mother" "Oh. That's alright. Sorry I'm not very used to humour." (`|MakeArray` "[Next]" :!type "Text")))
                      (switch `/Game/Blueprints/Enum_DialogueState` _state_53
                        (:`NewEnumerator0`
                          (bind _state_54 (`self.AddDialogue` "Mother" "I've been here a long time, and don't get to talk to people much. With my husband working all day, it's usually just me at home, and looking after Lily." (`|MakeArray` "Your daughter?" "Lily?" :!type "Text")))
                          (switch `/Game/Blueprints/Enum_DialogueState` _state_54
                            (:`NewEnumerator0`
                              (goto _label_2))))))
                    (:`1`
                      (bind _state_55 (`self.AddDialogue` "Mother" "..." (`|MakeArray` "[Close]" :!type "Text")))
                      (switch `/Game/Blueprints/Enum_DialogueState` _state_55
                        (:`NewEnumerator0`
                          (`self.ClearDialogueProgress`)
                          (`self.CloseConversation`))))))))
            (:`2`
              (bind (_state_56 _optionindex_7) (`self.AddDialogue` "Mother" "...Pleasantries, was there something else?" (`|MakeArray` "If you don't mind me asking.." "Nothing, nevermind" :!type "Text")))
              (switch `/Game/Blueprints/Enum_DialogueState` _state_56
                (:`NewEnumerator0`
                  (switch `int` _optionindex_7
                    (:`0`
                      (bind _state_57 (`self.AddDialogue` "Mother" "Yes?" (`|MakeArray` "Did you always want to be a mother?" "Didn't you want to have kids?" :!type "Text")))
                      (switch `/Game/Blueprints/Enum_DialogueState` _state_57
                        (:`NewEnumerator0`
                          (goto _label_3))))
                    (:`1`
                      (bind _state_58 (`self.AddDialogue` "Mother" "Pleasant day." (`|MakeArray` "[Close]" :!type "Text")))
                      (switch `/Game/Blueprints/Enum_DialogueState` _state_58
                        (:`NewEnumerator0`
                          (`self.ClearDialogueProgress`)
                          (`self.CloseConversation`))))))))
            (:`3`
              (bind (_state_59 _optionindex_8) (`self.AddDialogue` "Mother" "...Yes?" (`|MakeArray` "I'm sorry, tell me more" "Nothing, nevermind" :!type "Text")))
              (switch `/Game/Blueprints/Enum_DialogueState` _state_59
                (:`NewEnumerator0`
                  (switch `int` _optionindex_8
                    (:`0`
                      (bind _state_60 (`self.AddDialogue` "Mother" "...Are you sure I can trust you?" (`|MakeArray` "You can, I promise you" "I want change, just like you do" :!type "Text")))
                      (switch `/Game/Blueprints/Enum_DialogueState` _state_60
                        (:`NewEnumerator0`
                          (goto _label_4))))
                    (:`1`
                      (`self.ClearDialogueProgress`)
                      (`self.CloseConversation`))))))))))))